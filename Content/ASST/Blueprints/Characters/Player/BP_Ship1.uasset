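; BP_Ship1 is a player ship Blueprint that layers ship-specific startup settings on top of its parent class.
; On BeginPlay it runs the parent logic, raises the All-Range Mode speed and saves it as the default.
; It also caches the ship mesh's base material and grants a starting stock of bombs.
; Tick and the construction script only call the parent versions.
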(event EventBeginPlay
  (|CallParentFunction)
  ;[1 1 1] Make New Speed 25 (up from 10)
  (Variables|Default|SetAllRangeModeSpeed 25.0)
  ;;[1 1 1] Save All-Range Mode speed
  (Variables|Default|SetDefaultAllRangeSpeed (Variables|Default|GetAllRangeModeSpeed))
  ;[1 1 1] Save BaseColor of Ship
  (Variables|Default|SetBaseColorMaterial (Rendering|Material|GetMaterial (Variables|Default|GetShip) 0))
  ;[1 1 1] Start with 5 bombs
  (CallFunction|FnAddBombs 5))

(event Collision|EventActorBeginOverlap
  (params (OtherActor :type Actor%20Object%20Reference)))

(event EventTick
  (params (DeltaSeconds :type Float%20%28single-precision%29))
  (|CallParentFunction DeltaSeconds))

(fn ConstructionScript
  (|CallParentFunction))