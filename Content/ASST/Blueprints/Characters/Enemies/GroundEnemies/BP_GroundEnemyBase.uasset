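; BP_GroundEnemyBase is a base Blueprint for ground enemies, providing lock-on feedback and a reset to the enemy's starting state.
; BeginPlay saves the actor's starting location and rotation.
; fnLocked and fnUnlocked show and hide the LockTargetReticule component.
; fnReset deactivates the enemy and teleports it back to the saved transform.
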(event EventBeginPlay
  ;[1 1 1] Save starting location and rotation for fnReset
  (Variables|Default|SetSavedStartLocation (Transformation|GetActorLocation))
  (Variables|Default|SetSavedStartRotation (Transformation|GetActorRotation)))

(fn ConstructionScript)

(fn FnLocked
  ;[1 1 1] Show target reticule
  (Rendering|SetVisibility (Variables|Default|GetLockTargetReticule) true false))

(fn FnUnlocked
  ;[1 1 1] Hide reticule
  (Rendering|SetVisibility (Variables|Default|GetLockTargetReticule) false false))

(fn FnReset
  ;[1 1 1] Deactive enemy
  (Variables|Default|SetEnemyActive false)
  ;[1 1 1] Reset actor location and rotation
  (Transformation|SetActorLocationAndRotation (Variables|Default|GetSavedStartLocation) (Variables|Default|GetSavedStartRotation) false true))