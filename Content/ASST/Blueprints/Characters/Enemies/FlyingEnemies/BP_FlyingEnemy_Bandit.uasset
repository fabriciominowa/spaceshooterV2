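; Bandit flying enemy Blueprint that fires twin projectiles at the player's ship, building on a parent enemy class.
; BeginPlay sets the obstacle-avoidance collision radius, and construction sets the death delay.
; EventFire maps damage type to a projectile tag, then spawns lasers or fireballs from left and right spawn points, aimed at the player.
; Projectile type can make each shot home in on the ship or trigger its never-miss event.
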(event EventBeginPlay
  (|CallParentFunction)
  ;[1 1 1] Collision radius used for obstacle avoidance
  (Variables|Default|SetCollisionSphereRadius 2e+03))

(fn ConstructionScript
  (|CallParentFunction)
  ;[1 1 1] Set DM_DeathDelay to 10 - default in parentBP class
  (Variables|Default|SetDM_DeathDelay 1e+01))

(event EventEventFire
  (bind _spawnpointleft (Variables|Default|GetSpawnPointLeft))
  (bind _spawnpointright (Variables|Default|GetSpawnPointRight))
  (bind _spawnpointleft_2 (Variables|Default|GetSpawnPointLeft))
  (bind _spawnpointright_2 (Variables|Default|GetSpawnPointRight))
  (bind _returnvalue (Transformation|GetWorldLocation _spawnpointleft))
  (bind _returnvalue_2 (Transformation|GetWorldLocation _spawnpointright))
  (bind _returnvalue_3 (Transformation|GetWorldLocation _spawnpointleft_2))
  (bind _returnvalue_4 (Transformation|GetWorldLocation _spawnpointright_2))
  ;[1 1 1] Choose damage type
  (switch Utilities|FlowControl|Switch|SwitchonEnum_DamageType (Variables|Default|GetDamageType)
    (:NewEnumerator0
      ;[1 1 1] Set projectile tag
      (Variables|Default|SetProjectileTag (Variables|Default|GetCrashTag)))
    (:NewEnumerator1
      (Variables|Default|SetProjectileTag (Variables|Default|GetLightTag)))
    (:NewEnumerator2
      (Variables|Default|SetProjectileTag (Variables|Default|GetHeavyTag)))
    (:NewEnumerator3
      (Variables|Default|SetProjectileTag (Variables|Default|GetShieldBreakTag)))
    (:NewEnumerator4
      (Variables|Default|SetProjectileTag (Variables|Default|GetInstaDeathTag))))
  ;[1 1 1] Select weapon type
  (switch Utilities|FlowControl|Switch|SwitchonEnum_WeaponType (Variables|Default|GetWeaponType)
    (:NewEnumerator0
      (Utilities|FlowControl|Sequence
        (:then_0
          ;[1 1 1] Spawn Left Laser
          (bind _returnvalue_5 (Game|SpawnActorfromClass "/Game/ASST/Blueprints/Actors/Weapons/EnemyWeapons/BP_EnemyLaser.BP_EnemyLaser_C" (Math|Transform|MakeTransform (+ _returnvalue "100.000000, 0, 0") (Math|Rotator|FindLookatRotation _returnvalue (Transformation|GetWorldLocation (Variables|/Game/ASST/Blueprints/Characters/Player/BP_PlayerShip.BP_PlayerShip_C|GetRoot (Variables|Default|GetPlayerRef)))) "10.000000,10.000000,10.000000") "AdjustIfPossibleButAlwaysSpawn" 0 0))
          (Variables|/Script/Engine.Actor|SetTags _returnvalue_5 (Variables|Default|GetProjectileTag))
          (switch Utilities|FlowControl|Switch|SwitchonEnum_EnemyProjectileType (Variables|Default|GetProjectileType)
            (:NewEnumerator1
              ;[1 1 1] Make projectile a homing projectile
              (bind _asbp_player_ship (Utilities|Casting|CastToBP_PlayerShip (Game|Player|GetPlayerPawn 0)))
              (Variables|/Script/Engine.ProjectileMovementComponent|SetHomingTargetComponent (Variables|/Game/ASST/Blueprints/Actors/Weapons/EnemyWeapons/BP_EnemyLaser.BP_EnemyLaser_C|GetProjectileMovement _returnvalue_5) (Variables|/Game/ASST/Blueprints/Characters/Player/BP_PlayerShip.BP_PlayerShip_C|GetRoot _asbp_player_ship))
              (Variables|/Script/Engine.ProjectileMovementComponent|SetbIsHomingProjectile (Variables|/Game/ASST/Blueprints/Actors/Weapons/EnemyWeapons/BP_EnemyLaser.BP_EnemyLaser_C|GetProjectileMovement _returnvalue_5) true)
              (Variables|/Script/Engine.ProjectileMovementComponent|SetHomingAccelerationMagnitude (Variables|/Game/ASST/Blueprints/Actors/Weapons/EnemyWeapons/BP_EnemyLaser.BP_EnemyLaser_C|GetProjectileMovement _returnvalue_5) 4e+04))
            (:NewEnumerator2
              ;[1 1 1] Call EventNeverMiss and pass Player
              (Default|EventNeverMiss _returnvalue_5 (Game|Player|GetPlayerPawn 0)))))
        (:then_1
          ;[1 1 1] Spawn Right Laser
          (bind _returnvalue_6 (Game|SpawnActorfromClass "/Game/ASST/Blueprints/Actors/Weapons/EnemyWeapons/BP_EnemyLaser.BP_EnemyLaser_C" (Math|Transform|MakeTransform (+ _returnvalue_2 "100.000000, 0, 0") (Math|Rotator|FindLookatRotation _returnvalue_2 (Transformation|GetWorldLocation (Variables|/Game/ASST/Blueprints/Characters/Player/BP_PlayerShip.BP_PlayerShip_C|GetRoot (Variables|Default|GetPlayerRef)))) "10.000000,10.000000,10.000000") "AdjustIfPossibleButAlwaysSpawn" 0 0))
          (Variables|/Script/Engine.Actor|SetTags _returnvalue_6 (Variables|Default|GetProjectileTag))
          (switch Utilities|FlowControl|Switch|SwitchonEnum_EnemyProjectileType (Variables|Default|GetProjectileType)
            (:NewEnumerator1
              ;[1 1 1] Make projectile a homing projectile
              (bind _asbp_player_ship_2 (Utilities|Casting|CastToBP_PlayerShip (Game|Player|GetPlayerPawn 0)))
              (Variables|/Script/Engine.ProjectileMovementComponent|SetHomingTargetComponent (Variables|/Game/ASST/Blueprints/Actors/Weapons/EnemyWeapons/BP_EnemyLaser.BP_EnemyLaser_C|GetProjectileMovement _returnvalue_6) (Variables|/Game/ASST/Blueprints/Characters/Player/BP_PlayerShip.BP_PlayerShip_C|GetRoot _asbp_player_ship_2))
              (Variables|/Script/Engine.ProjectileMovementComponent|SetbIsHomingProjectile (Variables|/Game/ASST/Blueprints/Actors/Weapons/EnemyWeapons/BP_EnemyLaser.BP_EnemyLaser_C|GetProjectileMovement _returnvalue_6) true)
              (Variables|/Script/Engine.ProjectileMovementComponent|SetHomingAccelerationMagnitude (Variables|/Game/ASST/Blueprints/Actors/Weapons/EnemyWeapons/BP_EnemyLaser.BP_EnemyLaser_C|GetProjectileMovement _returnvalue_6) 4e+04))
            (:NewEnumerator2
              ;[1 1 1] Call EventNeverMiss and pass Player
              (Default|EventNeverMiss _returnvalue_6 (Game|Player|GetPlayerPawn 0)))))))
    (:NewEnumerator1
      (Utilities|FlowControl|Sequence
        (:then_0
          ;[1 1 1] Spawn Left Fireball
          (bind _returnvalue_7 (Game|SpawnActorfromClass "/Game/ASST/Blueprints/Actors/Weapons/EnemyWeapons/BP_EnemyFireball.BP_EnemyFireball_C" (Math|Transform|MakeTransform _returnvalue_3 (Math|Rotator|FindLookatRotation _returnvalue_3 (Transformation|GetWorldLocation (Variables|/Game/ASST/Blueprints/Characters/Player/BP_PlayerShip.BP_PlayerShip_C|GetRoot (Variables|Default|GetPlayerRef)))) "5.000000,5.000000,5.000000") "AdjustIfPossibleButAlwaysSpawn" 0 0))
          (Variables|/Script/Engine.Actor|SetTags _returnvalue_7 (Variables|Default|GetProjectileTag))
          (switch Utilities|FlowControl|Switch|SwitchonEnum_EnemyProjectileType (Variables|Default|GetProjectileType)
            (:NewEnumerator1
              ;[1 1 1] Make projectile a homing projectile
              (bind _asbp_player_ship_3 (Utilities|Casting|CastToBP_PlayerShip (Game|Player|GetPlayerPawn 0)))
              (Variables|/Script/Engine.ProjectileMovementComponent|SetHomingTargetComponent (Variables|/Game/ASST/Blueprints/Actors/Weapons/EnemyWeapons/BP_EnemyFireball.BP_EnemyFireball_C|GetProjectileMovement _returnvalue_7) (Variables|/Game/ASST/Blueprints/Characters/Player/BP_PlayerShip.BP_PlayerShip_C|GetRoot _asbp_player_ship_3))
              (Variables|/Script/Engine.ProjectileMovementComponent|SetbIsHomingProjectile (Variables|/Game/ASST/Blueprints/Actors/Weapons/EnemyWeapons/BP_EnemyFireball.BP_EnemyFireball_C|GetProjectileMovement _returnvalue_7) true)
              (Variables|/Script/Engine.ProjectileMovementComponent|SetHomingAccelerationMagnitude (Variables|/Game/ASST/Blueprints/Actors/Weapons/EnemyWeapons/BP_EnemyFireball.BP_EnemyFireball_C|GetProjectileMovement _returnvalue_7) 4e+04))
            (:NewEnumerator2
              ;[1 1 1] Call EventNeverMiss and pass Player
              (Default|EventNeverMiss _returnvalue_7 (Game|Player|GetPlayerPawn 0)))))
        (:then_1
          ;[1 1 1] Spawn Right Fireball
          (bind _returnvalue_8 (Game|SpawnActorfromClass "/Game/ASST/Blueprints/Actors/Weapons/EnemyWeapons/BP_EnemyFireball.BP_EnemyFireball_C" (Math|Transform|MakeTransform _returnvalue_4 (Math|Rotator|FindLookatRotation _returnvalue_4 (Transformation|GetWorldLocation (Variables|/Game/ASST/Blueprints/Characters/Player/BP_PlayerShip.BP_PlayerShip_C|GetRoot (Variables|Default|GetPlayerRef)))) "5.000000,5.000000,5.000000") "AdjustIfPossibleButAlwaysSpawn" 0 0))
          (Variables|/Script/Engine.Actor|SetTags _returnvalue_8 (Variables|Default|GetProjectileTag))
          (switch Utilities|FlowControl|Switch|SwitchonEnum_EnemyProjectileType (Variables|Default|GetProjectileType)
            (:NewEnumerator1
              ;[1 1 1] Make projectile a homing projectile
              (bind _asbp_player_ship_4 (Utilities|Casting|CastToBP_PlayerShip (Game|Player|GetPlayerPawn 0)))
              (Variables|/Script/Engine.ProjectileMovementComponent|SetHomingTargetComponent (Variables|/Game/ASST/Blueprints/Actors/Weapons/EnemyWeapons/BP_EnemyFireball.BP_EnemyFireball_C|GetProjectileMovement _returnvalue_8) (Variables|/Game/ASST/Blueprints/Characters/Player/BP_PlayerShip.BP_PlayerShip_C|GetRoot _asbp_player_ship_4))
              (Variables|/Script/Engine.ProjectileMovementComponent|SetbIsHomingProjectile (Variables|/Game/ASST/Blueprints/Actors/Weapons/EnemyWeapons/BP_EnemyFireball.BP_EnemyFireball_C|GetProjectileMovement _returnvalue_8) true)
              (Variables|/Script/Engine.ProjectileMovementComponent|SetHomingAccelerationMagnitude (Variables|/Game/ASST/Blueprints/Actors/Weapons/EnemyWeapons/BP_EnemyFireball.BP_EnemyFireball_C|GetProjectileMovement _returnvalue_8) 4e+04))
            (:NewEnumerator2
              ;[1 1 1] Call EventNeverMiss and pass Player
              (Default|EventNeverMiss _returnvalue_8 (Game|Player|GetPlayerPawn 0)))))))))