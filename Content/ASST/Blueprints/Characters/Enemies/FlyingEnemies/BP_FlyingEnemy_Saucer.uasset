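; Flying saucer enemy that spins its ship mesh and fires projectiles at the player.
; A self-restarting timeline drives the yaw spin, and the construction script overrides the parent's death delay.
; EventFire maps damage type to a projectile tag, then spawns either a player-aimed laser or a mesh-oriented fireball.
; The projectile type can then make the shot home on the player or trigger its never-miss event.
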(event Custom|EventRotateShip
  (bind _yaw (Timeline|TM_Rotate PlayFromStart)
    (:Update
      ;[1 1 1] Update Yaw rotation
      (Transformation|SetRelativeRotation (Variables|Default|GetShip) (Math|Rotator|MakeRotator 0.0 0.0 _yaw) false false))
    (:Finished
      ;[1 1 1] Call event again when done rotating
      (CallFunction|EventRotateShip))))

(event EventBeginPlay
  (|CallParentFunction)
  ;[1 1 1] Set Rotation PlayRate for TMRotate
  (Components|Timeline|SetPlayRate (Variables|Default|GetTM_Rotate) (Variables|Setup-General|GetRotationPlayRate))
  ;[1 1 1] Rotate Ship
  (CallFunction|EventRotateShip))

(fn ConstructionScript
  (|CallParentFunction)
  ;[1 1 1] Set DM_DeathDelay to 10 - default in parentBP class
  (Variables|Default|SetDM_DeathDelay 1e+01))

(event EventEventFire
  (bind _spawnpoint (Variables|Default|GetSpawnPoint))
  (bind _returnvalue (Transformation|GetWorldLocation _spawnpoint))
  ;[1 1 1] Set Damage Type
  (switch Utilities|FlowControl|Switch|SwitchonEnum_DamageType (Variables|Default|GetDamageType)
    (:NewEnumerator0
      ;[1 1 1] Assign correct tag to projectile
      (Variables|Default|SetProjectileTag (Variables|Default|GetCrashTag)))
    (:NewEnumerator1
      (Variables|Default|SetProjectileTag (Variables|Default|GetLightTag)))
    (:NewEnumerator2
      (Variables|Default|SetProjectileTag (Variables|Default|GetHeavyTag)))
    (:NewEnumerator3
      (Variables|Default|SetProjectileTag (Variables|Default|GetShieldBreakTag)))
    (:NewEnumerator4
      (Variables|Default|SetProjectileTag (Variables|Default|GetInstaDeathTag))))
  ;[1 1 1] Set Weapon Type
  (switch Utilities|FlowControl|Switch|SwitchonEnum_WeaponType (Variables|Default|GetWeaponType)
    (:NewEnumerator0
      ;[1 1 1] Spawn Laser and add tag
      (bind _returnvalue_2 (Game|SpawnActorfromClass "/Game/ASST/Blueprints/Actors/Weapons/EnemyWeapons/BP_EnemyLaser.BP_EnemyLaser_C" (Math|Transform|MakeTransform (+ _returnvalue "100.000000, 0, 0") (Math|Rotator|FindLookatRotation _returnvalue (Transformation|GetWorldLocation (Variables|/Game/ASST/Blueprints/Characters/Player/BP_PlayerShip.BP_PlayerShip_C|GetRoot (Variables|Default|GetPlayerRef)))) "10.000000,15.000000,15.000000") "AdjustIfPossibleButAlwaysSpawn" 0 0))
      (Variables|Default|SetSpawnedLaser _returnvalue_2)
      (Variables|/Script/Engine.Actor|SetTags _returnvalue_2 (Variables|Default|GetProjectileTag))
      ;[1 1 1] Set projectile type
      (switch Utilities|FlowControl|Switch|SwitchonEnum_EnemyProjectileType (Variables|Default|GetProjectileType)
        (:NewEnumerator1
          ;[1 1 1] Make projectile a homing projectile
          (bind _asbp_player_ship (Utilities|Casting|CastToBP_PlayerShip (Game|Player|GetPlayerPawn 0)))
          (Variables|/Script/Engine.ProjectileMovementComponent|SetHomingTargetComponent (Variables|/Game/ASST/Blueprints/Actors/Weapons/EnemyWeapons/BP_EnemyLaser.BP_EnemyLaser_C|GetProjectileMovement (Variables|Default|GetSpawnedLaser)) (Variables|/Game/ASST/Blueprints/Characters/Player/BP_PlayerShip.BP_PlayerShip_C|GetRoot _asbp_player_ship))
          (Variables|/Script/Engine.ProjectileMovementComponent|SetbIsHomingProjectile (Variables|/Game/ASST/Blueprints/Actors/Weapons/EnemyWeapons/BP_EnemyLaser.BP_EnemyLaser_C|GetProjectileMovement (Variables|Default|GetSpawnedLaser)) true)
          (Variables|/Script/Engine.ProjectileMovementComponent|SetHomingAccelerationMagnitude (Variables|/Game/ASST/Blueprints/Actors/Weapons/EnemyWeapons/BP_EnemyLaser.BP_EnemyLaser_C|GetProjectileMovement (Variables|Default|GetSpawnedLaser)) 4e+04))
        (:NewEnumerator2
          ;[1 1 1] Call EventNeverMiss and pass Player
          (Default|EventNeverMiss (Variables|Default|GetSpawnedLaser) (Game|Player|GetPlayerPawn 0)))))
    (:NewEnumerator1
      ;[1 1 1] Spawn Fireball and add tag
      (bind _returnvalue_3 (Game|SpawnActorfromClass "/Game/ASST/Blueprints/Actors/Weapons/EnemyWeapons/BP_EnemyFireball.BP_EnemyFireball_C" (Math|Transform|MakeTransform (Transformation|GetWorldLocation (Variables|Default|GetSpawnPoint)) (Transformation|GetWorldRotation (Variables|Character|GetMesh)) "10.000000,10.000000,10.000000") "AdjustIfPossibleButAlwaysSpawn" 0 0))
      (Variables|Default|SetSpawnedFireball _returnvalue_3)
      (Variables|/Script/Engine.Actor|SetTags _returnvalue_3 (Variables|Default|GetProjectileTag))
      ;[1 1 1] Set projectile type
      (switch Utilities|FlowControl|Switch|SwitchonEnum_EnemyProjectileType (Variables|Default|GetProjectileType)
        (:NewEnumerator1
          ;[1 1 1] Make projectile a homing projectile
          (bind _asbp_player_ship_2 (Utilities|Casting|CastToBP_PlayerShip (Game|Player|GetPlayerPawn 0)))
          (Variables|/Script/Engine.ProjectileMovementComponent|SetHomingTargetComponent (Variables|/Game/ASST/Blueprints/Actors/Weapons/EnemyWeapons/BP_EnemyFireball.BP_EnemyFireball_C|GetProjectileMovement (Variables|Default|GetSpawnedFireball)) (Variables|/Game/ASST/Blueprints/Characters/Player/BP_PlayerShip.BP_PlayerShip_C|GetRoot _asbp_player_ship_2))
          (Variables|/Script/Engine.ProjectileMovementComponent|SetbIsHomingProjectile (Variables|/Game/ASST/Blueprints/Actors/Weapons/EnemyWeapons/BP_EnemyFireball.BP_EnemyFireball_C|GetProjectileMovement (Variables|Default|GetSpawnedFireball)) true)
          (Variables|/Script/Engine.ProjectileMovementComponent|SetHomingAccelerationMagnitude (Variables|/Game/ASST/Blueprints/Actors/Weapons/EnemyWeapons/BP_EnemyFireball.BP_EnemyFireball_C|GetProjectileMovement (Variables|Default|GetSpawnedFireball)) 4e+04))
        (:NewEnumerator2
          ;[1 1 1] Call EventNeverMiss and pass Player
          (Default|EventNeverMiss (Variables|Default|GetSpawnedFireball) (Game|Player|GetPlayerPawn 0)))))))