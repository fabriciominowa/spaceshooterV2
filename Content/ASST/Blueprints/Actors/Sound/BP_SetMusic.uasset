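; BP_SetMusic is a trigger actor that changes the background music when the player ship enters it.
; On overlap it accepts only actors of class BP_PlayerShip, waits StartDelay, then calls the ship's FnSetMusic with its configured track, ID and volume multiplier.
; The construction script writes its Text property to a TextRender component.
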(event OnComponentBeginOverlap(Trigger)
  (params (OverlappedComponent :type Primitive%20Component%20Object%20Reference) (OtherActor :type Actor%20Object%20Reference) (OtherComp :type Primitive%20Component%20Object%20Reference) (OtherBodyIndex :type Integer) (bFromSweep :type Boolean) (SweepResult :type Hit%20Result%20Structure%20%28by%20ref%29))
  ;[1 1 1] Only overlap Player
  (if (== (Utilities|GetClass OtherActor) "/Game/ASST/Blueprints/Characters/Player/BP_PlayerShip.BP_PlayerShip_C")
    ;[1 1 1] Wait StartDelay before proceeding
    (Utilities|FlowControl|Delay (Variables|Setup|GetStartDelay))
    ;[1 1 1] Cast to Player and set the new background music track
    (bind _asbp_player_ship (Utilities|Casting|CastToBP_PlayerShip OtherActor))
    (Default|FnSetMusic _asbp_player_ship (Variables|Setup|GetMusic) (Variables|Setup|GetMusicID) (Variables|Setup|GetVolumeMultiplier))))

(fn ConstructionScript
  (Rendering|Components|TextRender|SetText (Variables|Default|GetTextRender) (Variables|Setup|GetText)))