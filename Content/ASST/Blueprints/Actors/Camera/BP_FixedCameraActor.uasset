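; Camera actor that follows the player ship, registers itself with it and becomes the view target when the ship's fixed camera is active.
; Each Tick it runs All Range, Track or Stage Clear logic, or just looks at the ship once dead.
; Track mode rides the spline with damped panning, pitch and roll, watching somersaults from a static camera.
; Stage Clear can play timelines that orbit the ship, then switch to a front camera.
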(event EventBeginPlay
  ;[1 1 1] Save the Player reference
  (bind _asbp_player_ship (Utilities|Casting|CastToBP_PlayerShip (Game|Player|GetPlayerPawn 0)))
  (bind _output_get (Variables|Default|SetPlayerRef _asbp_player_ship))
  ;[1 1 1] Check if Player reference is valid
  (if (Utilities|IsValid _output_get)
    ;[1 1 1] Set Initial TargetLocation
    (Variables|Default|SetTargetLocation (Transformation|GetActorLocation (Variables|Default|GetPlayerRef)))
    ;[1 1 1] Set Initial TargetRotation
    (Variables|Default|SetTargetRotation (Transformation|GetActorRotation (Variables|Default|GetPlayerRef)))
    ;[1 1 1] Save the Max Z and Y values from Player
    (Variables|TrackMode|SetMaxZValue (Variables|/Game/ASST/Blueprints/Characters/Player/BP_PlayerShip.BP_PlayerShip_C|GetMaxZValue (Variables|Default|GetPlayerRef)))
    (Variables|TrackMode|SetMaxYValue (Variables|/Game/ASST/Blueprints/Characters/Player/BP_PlayerShip.BP_PlayerShip_C|GetMaxYValue (Variables|Default|GetPlayerRef)))
    ;[1 1 1] Set CameraActorRef to Self
    (Variables|/Game/ASST/Blueprints/Characters/Player/BP_PlayerShip.BP_PlayerShip_C|SetFixedCameraActorRef (Variables|Default|GetPlayerRef) self)
    ;[1 1 1] If this actor is active, set ViewTarget to self
    (if (Variables|/Game/ASST/Blueprints/Characters/Player/BP_PlayerShip.BP_PlayerShip_C|GetFixedCameraActive? (Variables|Default|GetPlayerRef))
      ;[1 1 1] Automatically set this camera as active
      (Game|Player|SetViewTargetwithBlend (Game|GetPlayerController 0) self 0.0 "VTBlend_Cubic" 0.0 false))))

(event EventTick
  (params (DeltaSeconds :type Float%20%28single-precision%29))
  ;[1 1 1] Check Player reference is valid
  (if (Utilities|IsValid (Variables|Default|GetPlayerRef))
    ;[1 1 1] Check if Player is NOT dead
    (if (not (Variables|/Game/ASST/Blueprints/Characters/Player/BP_PlayerShip.BP_PlayerShip_C|GetIsDead (Variables|Default|GetPlayerRef)))
      ;[1 1 1] Track player by using the appropriate method
      (switch Utilities|FlowControl|Switch|SwitchonEnum_CameraMode (Variables|Default|GetCameraMode)
        (:NewEnumerator0
          (CallFunction|EventAllRangeMode))
        (:NewEnumerator1
          (CallFunction|EventTrackMode))
        (:NewEnumerator2
          (CallFunction|EventStageClear)))
      (else
        ;[1 1 1] Player is dead - keep the camera in the same location but follow player
        (Transformation|SetActorRotation (Math|Rotator|FindLookatRotation (Transformation|GetActorLocation) (Transformation|GetActorLocation (Variables|Default|GetPlayerRef))))))))

(fn ConstructionScript)

(event Custom|EventStageClear
  (bind _playerref (Variables|Default|GetPlayerRef))
  (bind _springarm (Variables|Default|GetSpringArm))
  (bind _returnvalue (Transformation|GetActorLocation _playerref))
  ;[1 1 1] Check if Player is on a track
  (if (Variables|/Game/ASST/Blueprints/Characters/Player/BP_PlayerShip.BP_PlayerShip_C|GetTrackModeActive (Variables|Default|GetPlayerRef))
    ;[1 1 1] Track - Set actor location based on Player
    (Transformation|SetActorLocation _returnvalue false true)
    (else
      ;[1 1 1] ARM - set actor location and rotation based on Player
      (Transformation|SetActorLocationAndRotation _returnvalue (Transformation|GetActorRotation _playerref) false true)))
  ;[1 1 1] Rotate camera during sequence?
  (if (Variables|StageClear|GetRotateCamera?)
    (Utilities|FlowControl|DoOnce false
      (:Completed
        ;[1 1 1] Switch cameras to this actor
        (Game|Player|SetViewTargetwithBlend (Game|GetPlayerController 0) self 1.0 "VTBlend_Cubic" 0.0 false)
        ;[1 1 1] Set camera's relative location to z=80
        (Transformation|SetRelativeLocation (Variables|Default|GetCamera) "0, 0,80.000000" false true)
        (bind _alpha (Timeline|TM_RotateCamera Play)
          (:Update
            ;[1 1 1] Rotate camera 240 degrees around the ship
            (Transformation|SetRelativeRotation (Variables|Default|GetSpringArm) (Math|Rotator|MakeRotator 0.0 0.0 (Math|Float|Lerp 0.0 2.4e+02 _alpha)) false true)
            ;[1 1 1] Increase spring arm length
            (Variables|/Script/Engine.SpringArmComponent|SetTargetArmLength _springarm (+ (Variables|/Script/Engine.SpringArmComponent|GetTargetArmLength _springarm) 0.5)))
          (:Finished
            ;[1 1 1] Activate top camera
            (Components|Activation|SetActive (Variables|Default|GetCameraFront) true false)
            (Components|Activation|SetActive (Variables|Default|GetCamera) false false)
            (bind _alpha_2 (Timeline|TM_CloseUp Play)
              (:Update
                ;[1 1 1] Get camera closer to Player
                (Variables|/Script/Engine.SpringArmComponent|SetTargetArmLength (Variables|Default|GetSpringArm1) (Math|Float|Lerp 3e+02 4.5e+02 _alpha_2))))))))))

(event Custom|EventAllRangeMode
  (bind _playerref (Variables|Default|GetPlayerRef))
  (bind _playerref_2 (Variables|Default|GetPlayerRef))
  ;[1 1 1] Set camera's relative Z offset
  (Transformation|SetRelativeLocation (Variables|Default|GetCamera) (Math|Vector|MakeVector 0.0 0.0 (Variables|TrackMode|GetCameraZOffset)) false true)
  ;[1 1 1] Set actor's location and rotation based on Player
  (Transformation|SetActorLocationAndRotation (Transformation|GetActorLocation _playerref) (Transformation|GetActorRotation _playerref) false true)
  ;[1 1 1] If Player is doing a UTurn or Sommersault, Inherit Roll
  (if (or (Variables|/Game/ASST/Blueprints/Characters/Player/BP_PlayerShip.BP_PlayerShip_C|GetDoingSomersault? _playerref_2) (Variables|/Game/ASST/Blueprints/Characters/Player/BP_PlayerShip.BP_PlayerShip_C|GetDoingUTurn? _playerref_2))
    (Utilities|FlowControl|Sequence
      (:then_0
        (Utilities|FlowControl|DoOnce false :!label _label
          (:Completed
            (Variables|/Script/Engine.SpringArmComponent|SetbInheritRoll (Variables|Default|GetSpringArm) true)
            (Variables|/Script/Engine.SpringArmComponent|SetbEnableCameraRotationLag (Variables|Default|GetSpringArm) false))))
      (:then_1
        (goto _label_2 Reset)))
    (else
      (Utilities|FlowControl|Sequence
        (:then_0
          (Utilities|FlowControl|DoOnce false :!label _label_2
            (:Completed
              (Variables|/Script/Engine.SpringArmComponent|SetbInheritRoll (Variables|Default|GetSpringArm) false)
              (Variables|/Script/Engine.SpringArmComponent|SetbEnableCameraRotationLag (Variables|Default|GetSpringArm) true))))
        (:then_1
          (goto _label Reset))))))

(event Custom|EventTrackMode
  (bind _maxyvalue (Variables|TrackMode|GetMaxYValue))
  (bind _playerref (Variables|Default|GetPlayerRef))
  (bind _playerref_2 (Variables|Default|GetPlayerRef))
  (bind _camera (Variables|Default|GetCamera))
  (bind _camera_2 (Variables|Default|GetCamera))
  (bind _maxzvalue (Variables|TrackMode|GetMaxZValue))
  (bind _camera_3 (Variables|Default|GetCamera))
  (bind _camerapitch (Variables|TrackMode|GetCameraPitch))
  (bind _playerref_3 (Variables|Default|GetPlayerRef))
  (bind _returnvalue (- _maxzvalue 0.0))
  (bind _returnvalue_2 (- _maxyvalue 0.0))
  (bind _returnvalue_3 (Transformation|GetWorldRotation _camera))
  (bind _returnvalue_4 (Transformation|GetWorldRotation _camera_3))
  (bind _returnvalue_5 (Transformation|GetWorldRotation _camera_2))
  (bind _currenttrack (Variables|/Game/ASST/Blueprints/Characters/Player/BP_PlayerShip.BP_PlayerShip_C|GetCurrentTrack _playerref_2))
  (bind _playertracker (Variables|/Game/ASST/Blueprints/Actors/Tracks/BP_Track.BP_Track_C|GetPlayerTracker _currenttrack))
  (bind _returnvalue_6 (Transformation|GetWorldRotation _playertracker))
  ;[1 1 1] Check if Player is NOT doing a Somersault
  (if (not (Variables|/Game/ASST/Blueprints/Characters/Player/BP_PlayerShip.BP_PlayerShip_C|GetDoingSomersault? (Variables|Default|GetPlayerRef)))
    (Utilities|FlowControl|Sequence
      (:then_0
        ;[1 1 1] Check if we need to reset the camera rotation (after sommersault)
        (if (Variables|TrackMode|GetResetCameraRotation?)
          (Variables|TrackMode|SetResetCameraRotation? false)
          ;[1 1 1] Reset Relative Rotation
          (Transformation|SetRelativeRotation (Variables|Default|GetCamera) (Math|Rotator|MakeRotator 0.0 (Variables|TrackMode|GetCameraPitch) 0.0) false false)))
      (:then_1
        ;[1 1 1] Set actor location along the track (spline)
        (Transformation|SetActorLocation (Spline|GetLocationatDistanceAlongSpline (Variables|/Game/ASST/Blueprints/Actors/Tracks/BP_Track.BP_Track_C|GetSpline (Variables|/Game/ASST/Blueprints/Characters/Player/BP_PlayerShip.BP_PlayerShip_C|GetCurrentTrack _playerref)) (Variables|/Game/ASST/Blueprints/Characters/Player/BP_PlayerShip.BP_PlayerShip_C|GetDistanceAlongTrack _playerref) "World") false true)
        ;[1 1 1] Set Actor rotation based on track's PlayerTracker rotation
        (Transformation|SetActorRotation (Math|Rotator|MakeRotator (.roll (Transformation|GetWorldRotation (Variables|Default|GetCamera))) (.pitch _returnvalue_6) (.yaw _returnvalue_6)) true)
        ;[1 1 1] Offset Camera to 80% of Player's offset (camera panning)
        (Transformation|SetRelativeLocation (Variables|Default|GetCamera) (Math|Vector|MakeVector 0.0 (Math|Float|Clamp(Float) (* (Variables|/Game/ASST/Blueprints/Characters/Player/BP_PlayerShip.BP_PlayerShip_C|GetFTrackYOffset _playerref_3) 0.8) (* _returnvalue_2 -1.0) (* _returnvalue_2 1.0)) (+ (Math|Float|Clamp(Float) (* (Variables|/Game/ASST/Blueprints/Characters/Player/BP_PlayerShip.BP_PlayerShip_C|GetFTrackZOffset _playerref_3) 0.8) (* _returnvalue -1.0) (* _returnvalue 1.0)) (Variables|TrackMode|GetCameraZOffset))) false true)
        (if (Variables|TrackMode|GetRotateCameraBasedOnPitch?)
          ;[1 1 1] Determine if the Player is moving up or down
          (if (!= (Variables|/Game/ASST/Blueprints/Characters/Player/BP_PlayerShip.BP_PlayerShip_C|GetMoveUp (Variables|Default|GetPlayerRef)) 0.0)
            ;[1 1 1] Determine Player's pitch to rotate camera
            (if (> (.pitch (Transformation|GetActorRotation (Variables|Default|GetPlayerRef))) 0.0)
              ;[1 1 1] Calculate Target Pitch
              (Variables|TrackMode|SetTargetPitch (* _camerapitch -1.0))
              (else
                (Variables|TrackMode|SetTargetPitch _camerapitch)))
            ;[1 1 1] Rotate camera based on Player's pitch
            (Transformation|SetRelativeRotation (Variables|Default|GetCamera) (Math|Rotator|MakeRotator 0.0 (Math|Interpolation|FInterpTo (.pitch (Variables|/Script/Engine.SceneComponent|GetRelativeRotation (Variables|Default|GetCamera))) (Variables|TrackMode|GetTargetPitch) (Utilities|Time|GetWorldDeltaSeconds) 0.8) 0.0) false false)))
        ;[1 1 1] Determine if we need to adjust camera roll
        (if (Variables|TrackMode|GetUseCameraRoll?)
          ;[1 1 1] Moving right
          (if (> (Variables|/Game/ASST/Blueprints/Characters/Player/BP_PlayerShip.BP_PlayerShip_C|GetMoveRight (Variables|Default|GetPlayerRef)) 0.0)
            ;[1 1 1] Set roll to 5
            (Transformation|SetWorldRotation (Variables|Default|GetCamera) (Math|Rotator|MakeRotator (Math|Interpolation|FInterpTo (.roll _returnvalue_4) (Variables|TrackMode|GetCameraRollTarget) (Utilities|Time|GetWorldDeltaSeconds) (Variables|TrackMode|GetCameraInterpSpeed)) (.pitch _returnvalue_4) (.yaw _returnvalue_4)) false true)
            (else
              ;[1 1 1] Moving left
              (if (< (Variables|/Game/ASST/Blueprints/Characters/Player/BP_PlayerShip.BP_PlayerShip_C|GetMoveRight (Variables|Default|GetPlayerRef)) 0.0)
                ;[1 1 1] Set roll to -5
                (Transformation|SetWorldRotation (Variables|Default|GetCamera) (Math|Rotator|MakeRotator (Math|Interpolation|FInterpTo (.roll _returnvalue_3) (* (Variables|TrackMode|GetCameraRollTarget) -1.0) (Utilities|Time|GetWorldDeltaSeconds) (Variables|TrackMode|GetCameraInterpSpeed)) (.pitch _returnvalue_3) (.yaw _returnvalue_3)) false true)
                (else
                  ;[1 1 1] Set roll to 0
                  (Transformation|SetWorldRotation (Variables|Default|GetCamera) (Math|Rotator|MakeRotator (Math|Interpolation|FInterpTo (.roll _returnvalue_5) 0.0 (Utilities|Time|GetWorldDeltaSeconds) (Variables|TrackMode|GetCameraInterpSpeed)) (.pitch _returnvalue_5) (.yaw _returnvalue_5)) false true))))))))
    (else
      ;[1 1 1] Player is doing a Somersault, keep camera static and follow Player
      (Transformation|SetRelativeRotation (Variables|Default|GetCamera) (Math|Rotator|FindLookatRotation (Transformation|GetWorldLocation (Variables|Default|GetCamera)) (Transformation|GetActorLocation (Variables|Default|GetPlayerRef))) false false)
      ;[1 1 1] Set this variable to true, so once Player is done with Sommersault, camera rotation is reset
      (Variables|TrackMode|SetResetCameraRotation? true))))

(event Custom|EventCenterCamera
  (bind _playerref (Variables|Default|GetPlayerRef))
  ;[1 1 1] Set camera's relative location to its appropriate Z offset and set the appropriate pitch
  (Transformation|SetRelativeLocationAndRotation (Variables|Default|GetCamera) (Math|Vector|MakeVector 0.0 0.0 (Variables|TrackMode|GetCameraZOffset)) (Math|Rotator|MakeRotator 0.0 (Variables|TrackMode|GetCameraPitch) 0.0) false true)
  ;[1 1 1] Set actor location and rotation based on Player
  (Transformation|SetActorLocationAndRotation (Transformation|GetActorLocation _playerref) (Transformation|GetActorRotation _playerref) false true))