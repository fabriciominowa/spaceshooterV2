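; BP_EnableThrustMode is a level actor that switches the player ship into Thrust Mode when play begins.
; On BeginPlay it casts the player pawn to BP_PlayerShip and calls its enable function.
; It then overrides the ship's current and default All-Range Mode speeds and its current track speed with its own speed variables.
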(event EventBeginPlay
  ;[1 1 1] Cast to the PlayerShip and enable Thrust Mode
  (bind _asbp_player_ship (Utilities|Casting|CastToBP_PlayerShip (Game|Player|GetPlayerPawn 0)))
  (Variables|Default|SetPlayerRef _asbp_player_ship)
  (Default|FnEnableThrustMode (Variables|Default|GetPlayerRef))
  ;[1 1 1] Set ARM and Track mode speeds
  (Variables|/Game/ASST/Blueprints/Characters/Player/BP_PlayerShip.BP_PlayerShip_C|SetAllRangeModeSpeed (Variables|Default|GetPlayerRef) (Variables|Setup|GetAllRangeModeSpeed))
  (Variables|/Game/ASST/Blueprints/Characters/Player/BP_PlayerShip.BP_PlayerShip_C|SetDefaultAllRangeSpeed (Variables|Default|GetPlayerRef) (Variables|Setup|GetAllRangeModeSpeed))
  (Variables|/Game/ASST/Blueprints/Characters/Player/BP_PlayerShip.BP_PlayerShip_C|SetCurrentTrackSpeed (Variables|Default|GetPlayerRef) (Variables|Setup|GetTrackSpeed)))

(fn ConstructionScript)