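; BP_TimeAttackManager runs Time Attack mode, ending in game over when time runs out and, if item collection is enabled, stage clear when all items are gone.
; On BeginPlay it shows the WBP_TimeAttack HUD and can disable the player ship's shield regeneration.
; Self-bound looping timers tick the countdown and poll tagged actors for items left, updating the HUD and calling BP_PlayerShip's end-of-game events.
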(event Custom|EventStartCountDown
  (bind _returnvalue (Utilities|Time|SetTimerbyEvent (delegate Custom|EventStartCountDown) 1.0 true))
  (Variables|Default|SetCountDownHandler _returnvalue)
  (Math|Integer|DecrementInt (Variables|Setup|GetTimeLimit)
    (:%20%20
      (Default|FnSetTimer (Variables|Default|GetWBPTimeAttackRef) (Variables|Setup|GetTimeLimit))
      ;[1 1 1] Is the timer less than 1?
      (if (< (Variables|Setup|GetTimeLimit) 1)
        (Utilities|Time|PauseTimerbyHandle (Variables|Default|GetCountDownHandler))
        ;[1 1 1] Display Game Over Screen
        (bind _asbp_player_ship (Utilities|Casting|CastToBP_PlayerShip (Game|Player|GetPlayerPawn 0)))
        (Default|EventGameOver _asbp_player_ship 0.0 "NewEnumerator2")))))

(event Custom|EventCheckItemsLeft
  (bind _returnvalue (Utilities|Time|SetTimerbyEvent (delegate Custom|EventCheckItemsLeft) 0.5 true))
  (Variables|Default|SetItemTimerHandler _returnvalue)
  (bind _outactors (Actor|GetAllActorswithTag (Variables|Setup|GetItemTag)))
  ;[1 1 1] Check to see if there are any NO items left
  (if (not (Utilities|IsValid (Utilities|Array|Get(acopy) _outactors)))
    (Utilities|Time|PauseTimerbyHandle (Variables|Default|GetItemTimerHandler))
    ;[1 1 1] All items collected, Game Over
    (bind _asbp_player_ship (Utilities|Casting|CastToBP_PlayerShip (Game|Player|GetPlayerPawn 0)))
    (Default|EventStageClear _asbp_player_ship "Time Attack Clear!")
    (else
      ;[1 1 1] Display items left
      (Default|FnSetItemsLeft (Variables|Default|GetWBPTimeAttackRef) (Utilities|Array|Length _outactors)))))

(event EventBeginPlay
  ;[1 1 1] Create and show the Time Attack Widget
  (bind _returnvalue (UserInterface|CreateWidget "/Game/ASST/Blueprints/UMG/HUD/WBP_TimeAttack.WBP_TimeAttack_C"))
  (bind _output_get (Variables|Default|SetWBPTimeAttackRef _returnvalue))
  (UserInterface|Viewport|AddtoViewport _output_get 0)
  (Default|FnSetTimer (Variables|Default|GetWBPTimeAttackRef) (Variables|Setup|GetTimeLimit))
  ;[1 1 1] Start the countdown
  (CallFunction|EventStartCountDown)
  (if (Variables|Setup|GetCollectItems?)
    (Default|FnDisplayItems (Variables|Default|GetWBPTimeAttackRef))
    (CallFunction|EventCheckItemsLeft))
  (if (Variables|Setup|GetDisableRegenShield?)
    (bind _asbp_player_ship (Utilities|Casting|CastToBP_PlayerShip (Game|Player|GetPlayerPawn 0)))
    (Variables|/Game/ASST/Blueprints/Characters/Player/BP_PlayerShip.BP_PlayerShip_C|SetRegenerateShield? _asbp_player_ship false)))

(fn ConstructionScript)