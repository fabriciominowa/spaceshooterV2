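; BP_SurvivalModeManager runs a survival stage in which the player clears it by eliminating all actors with the enemy tag.
; BeginPlay creates the WBP_SurvivalMode widget, starts enemy checks and optionally disables range checking on the player HUD radar.
; A looping timer, re-set on each check, counts tagged actors to update the enemies-left display.
; When none remain, it pauses the timer, waits, then calls EventStageClear on BP_PlayerShip.
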(event Custom|EventCheckEnemies
  (bind _returnvalue (Utilities|Time|SetTimerbyEvent (delegate Custom|EventCheckEnemies) 0.5 true))
  (Variables|Default|SetCheckEnemiesTimer _returnvalue)
  (bind _outactors (Actor|GetAllActorswithTag (Variables|Setup|GetEnemyTag)))
  ;[1 1 1] Check to see if there are NO enemies left with the EnemyTag
  (if (not (Utilities|IsValid (Utilities|Array|Get(acopy) _outactors)))
    ;[1 1 1] Pause timer
    (Utilities|Time|PauseTimerbyHandle (Variables|Default|GetCheckEnemiesTimer))
    (Utilities|FlowControl|Delay (Variables|Setup|GetClearStageDelay))
    ;[1 1 1] No enemies left - Stage Clear
    (CallFunction|EventStageClear)
    (else
      ;[1 1 1] Enemies left, display counter
      (Default|FnSetEnemiesLeft (Variables|Default|GetWBPSurvivalRef) (Utilities|Array|Length _outactors)))))

(event Custom|EventStageClear
  ;[1 1 1] Cast to Player and call EventStageClear to go to the next level
  (bind _asbp_player_ship (Utilities|Casting|CastToBP_PlayerShip (Game|Player|GetPlayerPawn 0)))
  (Default|EventStageClear _asbp_player_ship (Variables|Setup|GetStageClearMessage)))

(event EventBeginPlay
  ;[1 1 1] Create and display Survival Mode widget
  (bind _returnvalue (UserInterface|CreateWidget "/Game/ASST/Blueprints/UMG/HUD/WBP_SurvivalMode.WBP_SurvivalMode_C"))
  (bind _output_get (Variables|Default|SetWBPSurvivalRef _returnvalue))
  (UserInterface|Viewport|AddtoViewport _output_get 0)
  ;[1 1 1] Check enemies
  (Utilities|FlowControl|Delay 0.5)
  (CallFunction|EventCheckEnemies)
  ;[1 1 1] Check if we want to limit the radar range
  (if (not (Variables|Setup|GetLimitRadarRange?))
    ;[1 1 1] Disable range checking on the radar
    (bind _asbp_player_ship (Utilities|Casting|CastToBP_PlayerShip (Game|Player|GetPlayerPawn 0)))
    (Variables|/Game/ASST/Blueprints/UMG/Radar/WBP_Radar.WBP_Radar_C|SetCheckRange? (Variables|/Game/ASST/Blueprints/UMG/HUD/WBP_HUD.WBP_HUD_C|GetWBP_Radar (Variables|/Game/ASST/Blueprints/Characters/Player/BP_PlayerShip.BP_PlayerShip_C|GetWBPHUDRef _asbp_player_ship)) false)))

(fn ConstructionScript)