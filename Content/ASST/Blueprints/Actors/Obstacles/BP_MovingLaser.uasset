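; Laser obstacle that can ping-pong between two locations, two rotations, or both while active.
; Construction script picks the mesh, scales nine beams to length and sets the actor's damage-type tag.
; It also records start and end transforms from the actor's editor placement, with end capture gated by flags.
; Forward and backward timelines call each other endlessly, lerping between those transforms with configurable delays and play rates.
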(event EventBeginPlay
  ;[1 1 1] Is the Laser active?
  (if (Variables|Setup-General|GetActive?)
    (Utilities|FlowControl|Sequence
      (:then_0
        ;[1 1 1] Do we move the Laser?
        (if (Variables|Setup-General|GetMove?)
          ;[1 1 1] Set Movement TM playrate
          (CallFunction|EventSetMovementPlayRate)
          ;[1 1 1] Move forward
          (CallFunction|EventMoveForward)))
      (:then_1
        ;[1 1 1] Do we rotate the Laser?
        (if (Variables|Setup-General|GetRotate?)
          ;[1 1 1] Set rotation TM playrate
          (CallFunction|EventRotatePlayRate)
          ;[1 1 1] Rotate forward
          (CallFunction|EventRotateForward))))))

(fn ConstructionScript
  ;[1 1 1] Switch on the mesh type
  (switch Utilities|FlowControl|Switch|SwitchonEnum_Laser_MeshType (Variables|Setup-General|GetMesh%20Type)
    (:NewEnumerator0
      ;[1 1 1] Set moving laser mesh
      (Components|StaticMesh|SetStaticMesh (Variables|Default|GetStaticMesh) (Variables|Default|GetMesh1)))
    (:NewEnumerator1
      ;[1 1 1] Set rotating laser mesh
      (Components|StaticMesh|SetStaticMesh (Variables|Default|GetStaticMesh) (Variables|Default|GetMesh2))))
  ;[1 1 1] Set laser beam length
  (Transformation|SetWorldScale3D (Variables|Default|GetBeam1) (Math|Vector|MakeVector 1.0 1.0 (Variables|Setup-General|GetBeamLength)))
  ;[1 1 1] Switch on damage type
  (switch Utilities|FlowControl|Switch|SwitchonEnum_DamageType (Variables|Setup-General|GetDamageType)
    (:NewEnumerator0
      ;[1 1 1] Set damage tags
      (Variables|Tags|SetBeamTag (Variables|Tags|GetCrashTag)))
    (:NewEnumerator1
      (Variables|Tags|SetBeamTag (Variables|Tags|GetLightTag)))
    (:NewEnumerator2
      (Variables|Tags|SetBeamTag (Variables|Tags|GetHeavyTag)))
    (:NewEnumerator3
      (Variables|Tags|SetBeamTag (Variables|Tags|GetShieldBreakTag)))
    (:NewEnumerator4
      (Variables|Tags|SetBeamTag (Variables|Tags|GetInstaDeathTag))))
  ;[1 1 1] Assign the damage tag to the actor
  (Variables|Default|SetTags (Variables|Tags|GetBeamTag))
  (Utilities|FlowControl|Sequence
    (:then_0
      ;[1 1 1] Did we capture the end location? If not save the final location
      (if (not (Variables|Setup-Movement|GetCaptureEndLocation))
        ;[1 1 1] Capture Final Location for Movement
        (Variables|Setup-Movement|SetFinalLocation (Transformation|GetActorLocation))
        (Utilities|FlowControl|Sequence :!label _label
          (:then_0
            ;[1 1 1] Did we capture the end rotation? If not save the final rotation
            (if (not (Variables|Setup-Rotation|GetCaptureEndRotation))
              ;[1 1 1] Capture Final Location for Movement
              (Variables|Setup-Rotation|SetFinalRotation (Transformation|GetActorRotation))))
          (:then_1
            ;[1 1 1] Set Starting location
            (Variables|Setup-Rotation|SetOriginalRotation (Transformation|GetActorRotation))))))
    (:then_1
      ;[1 1 1] Set Starting location
      (Variables|Setup-Movement|SetOriginalLocation (Transformation|GetActorLocation))
      (goto _label))))

(event Custom|EventRotateForward
  ;[1 1 1] Wait RotationStartDelay seconds
  (Utilities|FlowControl|Delay (Variables|Setup-Rotation|GetRotationStartDelay))
  ;[1 1 1] Move obstacle to location - TM is 2secs
  (bind _alpha (Timeline|TM_RotateForward PlayFromStart)
    (:Update
      (Transformation|SetActorRotation (Math|Rotator|Lerp(Rotator) (Variables|Setup-Rotation|GetOriginalRotation) (Variables|Setup-Rotation|GetFinalRotation) _alpha)))
    (:Finished
      (CallFunction|EventRotateBackwards))))

(event Custom|EventRotateBackwards
  ;[1 1 1] Wait RotationEndDelay seconds
  (Utilities|FlowControl|Delay (Variables|Setup-Rotation|GetRotationEndDelay))
  ;[1 1 1] Move obstacle to location - TM is 2secs
  (bind _alpha (Timeline|TM_RotateBackwards ReverseFromEnd)
    (:Update
      (Transformation|SetActorRotation (Math|Rotator|Lerp(Rotator) (Variables|Setup-Rotation|GetOriginalRotation) (Variables|Setup-Rotation|GetFinalRotation) _alpha)))
    (:Finished
      (CallFunction|EventRotateForward))))

(event Custom|EventRotatePlayRate
  ;[1 1 1] Set playrate to the rotation time lines
  (Components|Timeline|SetPlayRate (Variables|Default|GetTM_RotateForward) (Variables|Setup-Rotation|GetRotateForwardPlayRate))
  (Components|Timeline|SetPlayRate (Variables|Default|GetTM_RotateBackwards) (Variables|Setup-Rotation|GetRotateBackwardsPlayRate)))

(event Custom|EventMoveForward
  ;[1 1 1] Wait MovementStartDelay seconds
  (Utilities|FlowControl|Delay (Variables|Setup-Movement|GetMovementStartDelay))
  ;[1 1 1] Move obstacle to location - TM is 2secs
  (bind _alpha (Timeline|TM_Forward PlayFromStart)
    (:Update
      (Transformation|SetActorLocation (Math|Vector|Lerp(Vector) (Variables|Setup-Movement|GetOriginalLocation) (Variables|Setup-Movement|GetFinalLocation) _alpha) false false))
    (:Finished
      (CallFunction|EventMoveBackwards))))

(event Custom|EventMoveBackwards
  ;[1 1 1] Wait MovementEndDelay seconds
  (Utilities|FlowControl|Delay (Variables|Setup-Movement|GetMovementEndDelay))
  ;[1 1 1] Move obstacle to location - TM is 2secs
  (bind _alpha (Timeline|TM_Backwards ReverseFromEnd)
    (:Update
      (Transformation|SetActorLocation (Math|Vector|Lerp(Vector) (Variables|Setup-Movement|GetOriginalLocation) (Variables|Setup-Movement|GetFinalLocation) _alpha) false false))
    (:Finished
      (CallFunction|EventMoveForward))))

(event Custom|EventSetMovementPlayRate
  ;[1 1 1] Set play rate to the forward and backwards time lines
  (Components|Timeline|SetPlayRate (Variables|Default|GetTM_Forward) (Variables|Setup-Movement|GetForwardPlayRate))
  (Components|Timeline|SetPlayRate (Variables|Default|GetTM_Backwards) (Variables|Setup-Movement|GetBackwardsPlayRate)))