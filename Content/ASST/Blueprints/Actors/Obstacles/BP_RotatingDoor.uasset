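; Double-door obstacle actor that swings open when the player enters its trigger, if proximity opening is enabled, or when damage depletes its health.
; Damage subtracts from Health and briefly flashes both doors to a hurt material, firing the open event once at zero.
; The open event waits a configurable delay, then a timeline lerps both doors outward in opposite rotations.
; Construction script applies the base and accent materials.
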(event OnComponentBeginOverlap(Trigger)
  (params (OverlappedComponent :type Primitive%20Component%20Object%20Reference) (OtherActor :type Actor%20Object%20Reference) (OtherComp :type Primitive%20Component%20Object%20Reference) (OtherBodyIndex :type Integer) (bFromSweep :type Boolean) (SweepResult :type Hit%20Result%20Structure%20%28by%20ref%29))
  ;[1 1 1] Overlap only the Player
  (if (Actor|ActorHasTag OtherActor "Player")
    ;[1 1 1] Open the door on proximity?
    (if (Variables|Setup|GetOpenOnProximity?)
      ;[1 1 1] Open the doors
      (CallFunction|EventOpenDoors))))

(event EventBeginPlay
  ;[1 1 1] Set Timeline Playrate
  (Components|Timeline|SetPlayRate (Variables|Default|GetTM_OpenDoors) (Variables|Setup|GetPlayRate)))

(fn ConstructionScript
  (|CallParentFunction)
  ;[1 1 1] Set materials for the doors (index 0 and 1)
  (Rendering|Material|SetMaterial (Variables|Default|GetLeftDoor) 0 (Variables|Setup|GetBaseMaterial))
  (Rendering|Material|SetMaterial (Variables|Default|GetLeftDoor) 1 (Variables|Setup|GetAccentMaterial)))

(event Game|Damage|EventAnyDamage
  (params (Damage :type Float%20%28single-precision%29) (DamageType :type Damage%20Type%20Object%20Reference) (InstigatedBy :type Controller%20Object%20Reference) (DamageCauser :type Actor%20Object%20Reference))
  ;[1 1 1] Save damage taken and actor that hit
  (Variables|Default|SetDamageTaken Damage)
  (Variables|Default|SetActorThatHit DamageCauser)
  ;[1 1 1] Reduce Health by damage taken
  (Variables|Setup|SetHealth (- (Variables|Setup|GetHealth) (Variables|Default|GetDamageTaken)))
  (Utilities|FlowControl|Sequence
    (:then_0
      ;[1 1 1] Check if doors' Health is 0 or less
      (if (<= (Variables|Setup|GetHealth) 0.0)
        (Utilities|FlowControl|DoOnce false
          (:Completed
            ;[1 1 1] Open the doors
            (CallFunction|EventOpenDoors)))))
    (:then_1
      ;[1 1 1] Door is hit, change material to "Hurt" and after 0.1 seconds change back to normal material
      (Rendering|Material|SetMaterial (Variables|Default|GetLeftDoor) 0 (Variables|Setup|GetHurtMaterial))
      (Utilities|FlowControl|Delay 0.1)
      (Rendering|Material|SetMaterial (Variables|Default|GetLeftDoor) 0 (Variables|Setup|GetBaseMaterial)))))

(event Custom|EventOpenDoors
  ;[1 1 1] Wait OpenDelay seconds
  (Utilities|FlowControl|Delay (Variables|Setup|GetOpenDelay))
  (bind _alpha (Timeline|TM_OpenDoors PlayFromStart)
    (:Update
      ;[1 1 1] Lerp the rotation of the left door
      (Transformation|SetRelativeRotation (Variables|Default|GetLeftDoor) (Math|Rotator|Lerp(Rotator) "0, 0, 0" "0,-90.000000, 0" _alpha) false false)
      ;[1 1 1] Lerp the rotation of the right door
      (Transformation|SetRelativeRotation (Variables|Default|GetRightDoor) (Math|Rotator|Lerp(Rotator) "0, 0, 0" "0,90.000000, 0" _alpha) false false))))