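; Configurable obstacle for the player ship, with construction script setup of mesh, materials, trigger radius and a damage-type or environment tag.
; Two timelines with delays ping-pong it between captured start and end locations, optionally switching direction when the player hits it.
; Rotation runs constantly or while the player ship is inside the activation sphere.
; Entering that sphere can also enable physics with a standard, at-location or radial impulse.
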(event OnComponentBeginOverlap(ActivationTrigger)
  (params (OverlappedComponent :type Primitive%20Component%20Object%20Reference) (OtherActor :type Actor%20Object%20Reference) (OtherComp :type Primitive%20Component%20Object%20Reference) (OtherBodyIndex :type Integer) (bFromSweep :type Boolean) (SweepResult :type Hit%20Result%20Structure%20%28by%20ref%29))
  ;[1 1 1] Rotation Activation
  ;;[1 1 1] Only overlap Player
  (if (== (Utilities|GetClass OtherActor) "/Game/ASST/Blueprints/Characters/Player/BP_PlayerShip.BP_PlayerShip_C")
    ;;[1 1 1] Do we use rotation and is rotation NOT active?
    (if (and (Variables|Rotation|GetUseRotation?) (not (Variables|Rotation|GetRotationActive?)))
      ;;[1 1 1] Activate rotating movement
      (Components|Activation|Activate (Variables|Default|GetRotatingMovement) false))
    ;;[1 1 1] Do we simulate physics?
    (if (Variables|SimulatePhysics|GetSimulatePhysics?)
      ;;[1 1 1] Simulate physics
      (CallFunction|EventSimulatePhysics))))

(event OnComponentEndOverlap(ActivationTrigger)
  (params (OverlappedComponent :type Primitive%20Component%20Object%20Reference) (OtherActor :type Actor%20Object%20Reference) (OtherComp :type Primitive%20Component%20Object%20Reference) (OtherBodyIndex :type Integer))
  ;[1 1 1] Rotation Activation
  ;;[1 1 1] Only overlap Player
  (if (== (Utilities|GetClass OtherActor) "/Game/ASST/Blueprints/Characters/Player/BP_PlayerShip.BP_PlayerShip_C")
    ;;[1 1 1] Do we use rotation and is rotation NOT active?
    (if (and (Variables|Rotation|GetUseRotation?) (not (Variables|Rotation|GetRotationActive?)))
      ;;[1 1 1] Deactivate rotating movement
      (Components|Activation|Deactivate (Variables|Default|GetRotatingMovement)))))

(event EventBeginPlay
  ;[1 1 1] EVENT BEGIN PLAY
  (|CallParentFunction)
  (Utilities|FlowControl|Sequence
    (:then_0
      ;;[1 1 1] Is Obstacle active?
      (if (Variables|Rotation|GetRotationActive?)
        ;;[1 1 1] Activate rotating movement
        (Components|Activation|Activate (Variables|Default|GetRotatingMovement) false))
      ;;[1 1 1] If actor is part of the environment, Player will not pass through mesh when colliding
      ;;;[1 1 1] Is this part of the environment?
      (if (Variables|Setup|GetIsEnvironment?)
        ;;;[1 1 1] Set tag as 'Environment'
        (Variables|Default|SetTags (Variables|Tags|GetActorTags))))
    (:then_1
      ;;[1 1 1] Save starting location
      (Variables|Movement|SetOriginalLocation (Transformation|GetActorLocation))
      ;;[1 1 1] Set PlayRate and Start Movement
      (CallFunction|EventSetPlayRate)
      (CallFunction|EventForward))))

(fn ConstructionScript
  (|CallParentFunction)
  ;[1 1 1] Set activation radius
  (Components|Sphere|SetSphereRadius (Variables|Default|GetActivationTrigger) (Variables|Setup|GetActivationRadius) true)
  ;[1 1 1] Set rotation rate
  (Variables|/Script/Engine.RotatingMovementComponent|SetRotationRate (Variables|Default|GetRotatingMovement) (Variables|Rotation|GetRotationgRate))
  ;[1 1 1] Set mesh to use
  (Components|StaticMesh|SetStaticMesh (Variables|Character|GetMesh) (Variables|Mesh|GetObstacleMesh))
  ;[1 1 1] Set mesh scale
  (Transformation|SetWorldScale3D (Variables|Character|GetMesh) (Variables|Mesh|GetMeshScale))
  ;[1 1 1] Set mesh material
  (Rendering|Material|SetMaterial (Variables|Character|GetMesh) 0 (Variables|Mesh|GetMeshMaterial1))
  (Rendering|Material|SetMaterial (Variables|Character|GetMesh) 1 (Variables|Mesh|GetMeshMaterial2))
  ;[1 1 1] Switch on damage type
  (switch Utilities|FlowControl|Switch|SwitchonEnum_DamageType (Variables|Setup|GetDamageType)
    (:NewEnumerator0
      ;[1 1 1] Set damage tags based on damage
      (Variables|Tags|SetDamageTag (Variables|Tags|GetCrashTag)))
    (:NewEnumerator1
      (Variables|Tags|SetDamageTag (Variables|Tags|GetLightTag)))
    (:NewEnumerator2
      (Variables|Tags|SetDamageTag (Variables|Tags|GetHeavyTag)))
    (:NewEnumerator3
      (Variables|Tags|SetDamageTag (Variables|Tags|GetShieldBreakTag)))
    (:NewEnumerator4
      (Variables|Tags|SetDamageTag (Variables|Tags|GetInstaDeathTag))))
  ;[1 1 1] Assign the tag to the actor
  (Variables|Default|SetTags (Variables|Tags|GetDamageTag))
  (Utilities|FlowControl|Sequence
    (:then_0
      ;[1 1 1] Did we capture the end location? If not, save it
      (if (not (Variables|Movement|GetCaptureEndLocation))
        ;[1 1 1] Capture Final Location for Movement
        (Variables|Movement|SetFinalLocation (Transformation|GetActorLocation))))
    (:then_1
      ;[1 1 1] Set Starting location
      (Variables|Movement|SetOriginalLocation (Transformation|GetActorLocation)))))

(event Custom|EventSetPlayRate
  ;[1 1 1] Set the playrate for the forward and backwards time lines
  (Components|Timeline|SetPlayRate (Variables|Default|GetTM_Forward) (Variables|Movement|GetForwardPlayRate))
  (Components|Timeline|SetPlayRate (Variables|Default|GetTM_Backwards) (Variables|Movement|GetBackwardPlayRate)))

(event Custom|EventBackwards
  ;[1 1 1] Is the movement active?
  (if (Variables|Movement|GetMovementActive?)
    ;[1 1 1] Wait MovementBackDelay seconds
    (Utilities|FlowControl|Delay (Variables|Movement|GetMovementBackDelay))
    ;[1 1 1] Move obstacle to location - TM is 2secs
    (bind _alpha (Timeline|TM_Backwards ReverseFromEnd)
      (:Update
        (Transformation|SetActorLocation (Math|Vector|Lerp(Vector) (Variables|Movement|GetOriginalLocation) (Variables|Movement|GetFinalLocation) _alpha) false false))
      (:Finished
        (CallFunction|EventForward)))))

(event Custom|EventForward
  ;[1 1 1] Is the movement active?
  (if (Variables|Movement|GetMovementActive?)
    ;[1 1 1] Wait MovementStartDelay seconds
    (Utilities|FlowControl|Delay (Variables|Movement|GetMovementStartDelay))
    ;[1 1 1] Move obstacle to location - TM is 2secs
    (bind _alpha (Timeline|TM_Forward PlayFromStart)
      (:Update
        (Transformation|SetActorLocation (Math|Vector|Lerp(Vector) (Variables|Movement|GetOriginalLocation) (Variables|Movement|GetFinalLocation) _alpha) false false))
      (:Finished
        (CallFunction|EventBackwards)))))

(event Collision|EventHit
  (params (MyComp :type Primitive%20Component%20Object%20Reference) (Other :type Actor%20Object%20Reference) (OtherComp :type Primitive%20Component%20Object%20Reference) (bSelfMoved :type Boolean) (HitLocation :type Vector :default "0, 0, 0") (HitNormal :type Vector :default "0, 0, 0") (NormalImpulse :type Vector :default "0, 0, 0") (Hit :type Hit%20Result%20Structure%20%28by%20ref%29))
  ;[1 1 1] Were we hit by the Player?
  (if (Actor|ActorHasTag Other "Player")
    ;[1 1 1] Stop movement on impact?
    (if (Variables|Movement|GetStopMovementOnImpact?)
      ;[1 1 1] Is TM_Forward active?
      (if (Components|Activation|IsActive (Variables|Default|GetTM_Forward))
        ;[1 1 1] Stop moving forward and go backwards
        (Audio|Components|Audio|Stop (Variables|Default|GetTM_Forward))
        (CallFunction|EventBackwards)
        (else
          ;[1 1 1] Is TM_Backwards active?
          (if (Components|Activation|IsActive (Variables|Default|GetTM_Backwards))
            ;[1 1 1] Stop going backwards and go forward
            (Audio|Components|Audio|Stop (Variables|Default|GetTM_Backwards))
            (CallFunction|EventForward)))))))

(event Custom|EventSimulatePhysics
  ;[1 1 1] Do we simulate physics?
  (if (Variables|SimulatePhysics|GetSimulatePhysics?)
    ;[1 1 1] Simulate physics
    (Physics|SetSimulatePhysics (Variables|Character|GetMesh) true)
    ;[1 1 1] Do we add impulse?
    (if (Variables|SimulatePhysics|GetAddImpulse?)
      ;[1 1 1] Switch on impulse type
      (switch Utilities|FlowControl|Switch|SwitchonEnum_ImpulseType (Variables|SimulatePhysics|GetImpulseType)
        (:NewEnumerator0
          ;[1 1 1] Add normal impulse
          (Physics|AddImpulse (Variables|Character|GetMesh) (Variables|SimulatePhysics|GetImpulse) "None" false))
        (:NewEnumerator1
          ;[1 1 1] Add impulse at location
          (Physics|AddImpulseatLocation (Variables|Character|GetMesh) (Variables|SimulatePhysics|GetImpulse) (Variables|SimulatePhysics|GetImpulseLocation) "None"))
        (:NewEnumerator2
          ;[1 1 1] Add radial impulse
          (Physics|AddRadialImpulse (Variables|Character|GetMesh) (Variables|SimulatePhysics|GetImpulseLocation) (Variables|SimulatePhysics|GetRadialImpulseRadius) (Variables|SimulatePhysics|GetRadialImpulseStrength) "RIF_Constant" (Variables|SimulatePhysics|GetRadialImpulse_VelocityChange?)))))))