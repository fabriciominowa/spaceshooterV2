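; Destructible obstacle actor that can rotate, move and shatter when its health runs out.
; BeginPlay applies optional random rotation and scale; a timeline lerps it between start and end locations captured in the construction script, immediately or on player overlap.
; Hits stop rotation and store impact data for the fracture impulse, which is far stronger for radial damage.
; Destruction can play a pitch-varied sound, disable debris collision and destroy the actor.
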(event OnComponentBeginOverlap(ActivationTrigger)
  (params (OverlappedComponent :type Primitive%20Component%20Object%20Reference) (OtherActor :type Actor%20Object%20Reference) (OtherComp :type Primitive%20Component%20Object%20Reference) (OtherBodyIndex :type Integer) (bFromSweep :type Boolean) (SweepResult :type Hit%20Result%20Structure%20%28by%20ref%29))
  ;[1 1 1] Only overlap Player
  (if (Actor|ActorHasTag OtherActor "Player")
    ;[1 1 1] Activate movement and call Event Move
    (Variables|Movement|SetMovementActive? true)
    (CallFunction|EventMove)))

(event EventBeginPlay
  ;[1 1 1] Set rotation
  (if (Variables|Random|GetRandomRotation?)
    ;;[1 1 1] Set a random rotation based on the min and max ranges for each angle
    (Variables|/Script/Engine.RotatingMovementComponent|SetRotationRate (Variables|Default|GetRotatingMovement) (Math|Rotator|MakeRotator (Math|Random|RandomFloatinRange (Variables|Random|GetRotationMinRange) (Variables|Random|GetRotationMaxRange)) (Math|Random|RandomFloatinRange (Variables|Random|GetRotationMinRange) (Variables|Random|GetRotationMaxRange)) (Math|Random|RandomFloatinRange (Variables|Random|GetRotationMinRange) (Variables|Random|GetRotationMaxRange))))
    (else
      ;;[1 1 1] Set rotation rate to default
      (Variables|/Script/Engine.RotatingMovementComponent|SetRotationRate (Variables|Default|GetRotatingMovement) (Variables|Setup|GetRotationRate))))
  ;[1 1 1] Set random Scale
  (if (Variables|Random|GetRandomScale?)
    ;;[1 1 1] Set random scale based on the min and max ranges specified
    (Transformation|SetWorldScale3D (Variables|Default|GetDestructible) (Math|Vector|MakeVector (Math|Random|RandomFloatinRange (Variables|Random|GetScaleMinRange) (Variables|Random|GetScaleMaxRange)) (Math|Random|RandomFloatinRange (Variables|Random|GetScaleMinRange) (Variables|Random|GetScaleMaxRange)) (Math|Random|RandomFloatinRange (Variables|Random|GetScaleMinRange) (Variables|Random|GetScaleMaxRange)))))
  ;[1 1 1] Set PlayRate and call Move Event
  (CallFunction|EventSetPlayRate)
  (if (Variables|Movement|GetMoveImmediately?)
    (CallFunction|EventMove)))

(fn ConstructionScript
  (|CallParentFunction)
  ;[1 1 1] Set Mesh properties - mesh and materials
  (Class|DestructibleComponent|SetDestructibleMesh (Variables|Default|GetDestructible) (Variables|Setup|GetDestructibleMesh))
  (Rendering|Material|SetMaterial (Variables|Default|GetDestructible) 0 (Variables|Setup|GetOutsideMaterial))
  (Rendering|Material|SetMaterial (Variables|Default|GetDestructible) 1 (Variables|Setup|GetInsideMaterial))
  ;[1 1 1] Set the scale of the activation trigger
  (Transformation|SetWorldScale3D (Variables|Default|GetActivationTrigger) (Variables|Setup|GetActivationTriggerScale))
  ;[1 1 1] Set actor tags
  (Variables|Default|SetTags (Variables|Setup|GetActorTags))
  (Utilities|FlowControl|Sequence
    (:then_0
      ;[1 1 1] Did we capture the end location? If not, save end location
      (if (not (Variables|Movement|GetCapturedEnd))
        ;[1 1 1] Save end location
        (if (Variables|Movement|GetCaptureEndLocation)
          (Variables|Movement|SetEndLocation (Transformation|GetActorLocation)))))
    (:then_1
      ;[1 1 1] Save start location
      (if (Variables|Movement|GetCaptureStartLocation)
        (Variables|Movement|SetStartLocation (Transformation|GetActorLocation))))))

(event OnComponentHit(Destructible)
  (params (HitComponent :type Primitive%20Component%20Object%20Reference) (OtherActor :type Actor%20Object%20Reference) (OtherComp :type Primitive%20Component%20Object%20Reference) (NormalImpulse :type Vector :default "0, 0, 0") (Hit :type Hit%20Result%20Structure%20%28by%20ref%29))
  (bind (_bblockinghit _binitialoverlap _time _distance _location _impactpoint _normal _impactnormal) (Collision|BreakHitResult Hit))
  ;[1 1 1] Save impact location and normal
  (Variables|Default|SetImpactLocation _location)
  (Variables|Default|SetImpactNormal _impactnormal)
  ;[1 1 1] Deactivate the Movement Component
  (Components|Activation|Deactivate (Variables|Default|GetRotatingMovement)))

(event Game|Damage|EventAnyDamage
  (params (Damage :type Float%20%28single-precision%29) (DamageType :type Damage%20Type%20Object%20Reference) (InstigatedBy :type Controller%20Object%20Reference) (DamageCauser :type Actor%20Object%20Reference))
  ;[1 1 1] Save damage taken and actor that hit
  (Variables|Health|SetDamageTaken Damage)
  (Variables|Health|SetActorThatHit DamageCauser)
  ;[1 1 1] Reduce Health by damage taken
  (Variables|Health|SetHealth (- (Variables|Health|GetHealth) (Variables|Health|GetDamageTaken)))
  ;[1 1 1] If Health is 0 or less
  (if (<= (Variables|Health|GetHealth) 0.0)
    (Utilities|FlowControl|Sequence
      (:then_0
        (Utilities|FlowControl|DoOnce false
          (:Completed
            (if (Variables|Sound|GetPlaySound?)
              ;[1 1 1] Play destruction sound with small pitch variation
              (Audio|PlaySoundatLocation (Variables|Sound|GetDestructionSound) (Transformation|GetActorLocation) "0, 0, 0" 1.0 (Math|Random|RandomFloatinRange 0.7 1.2))))))
      (:then_1
        ;[1 1 1] Destroy Mesh
        ;;[1 1 1] Start simulating physics
        (Physics|SetSimulatePhysics (Variables|Default|GetDestructible) true)
        ;;[1 1 1] Disable hard sleeping of destructible mesh
        (Variables|/Script/ApexDestruction.DestructibleComponent|SetbEnableHardSleeping (Variables|Default|GetDestructible) false)
        ;;[1 1 1] Apply damage to the destructible mesh
        (Class|DestructibleComponent|ApplyDamage (Variables|Default|GetDestructible) (Variables|Health|GetDamageAmount) (Variables|Default|GetImpactLocation) (* (Variables|Default|GetImpactNormal) -1.0) (Variables|Health|GetImpulseStrength))
        ;;[1 1 1] Does debris have collision?
        (if (not (Variables|Setup|GetDebrisHasCollision?))
          ;;[1 1 1] Wait 0.5secs and disable collision
          (Utilities|FlowControl|Delay 0.5)
          (Collision|SetCollisionEnabled (Variables|Default|GetDestructible) "NoCollision"))
        ;[1 1 1] Destroy Actor
        ;;[1 1 1] Destroy the destructible actor?
        (if (Variables|Setup|GetDestroyActor?)
          ;;[1 1 1] Wait DestroyDelay seconds and destroy the actor
          (Utilities|FlowControl|Delay (Variables|Setup|GetDestroyDelay))
          (Actor|DestroyActor))))))

(event Game|Damage|EventRadialDamage
  (params (DamageReceived :type Float%20%28single-precision%29) (DamageType :type Damage%20Type%20Object%20Reference) (Origin :type Vector :default "0, 0, 0") (HitInfo :type Hit%20Result%20Structure%20%28by%20ref%29) (InstigatedBy :type Controller%20Object%20Reference) (DamageCauser :type Actor%20Object%20Reference))
  ;[1 1 1] Save damage taken and actor that hit
  (Variables|Health|SetDamageTaken DamageReceived)
  (Variables|Health|SetActorThatHit DamageCauser)
  ;[1 1 1] Reduce Health by damage taken
  (Variables|Health|SetHealth (- (Variables|Health|GetHealth) (Variables|Health|GetDamageTaken)))
  ;[1 1 1] If Health is 0 or less
  (if (<= (Variables|Health|GetHealth) 0.0)
    (Utilities|FlowControl|Sequence
      (:then_0
        (Utilities|FlowControl|DoOnce false
          (:Completed
            (if (Variables|Sound|GetPlaySound?)
              ;[1 1 1] Play destruction sound with small pitch variation
              (Audio|PlaySoundatLocation (Variables|Sound|GetDestructionSound) (Transformation|GetActorLocation) "0, 0, 0" 1.0 (Math|Random|RandomFloatinRange 0.7 1.2))))))
      (:then_1
        ;[1 1 1] Destroy Mesh
        ;;[1 1 1] Start simulating physics
        (Physics|SetSimulatePhysics (Variables|Default|GetDestructible) true)
        ;;[1 1 1] Disable hard sleeping of destructible mesh
        (Variables|/Script/ApexDestruction.DestructibleComponent|SetbEnableHardSleeping (Variables|Default|GetDestructible) false)
        ;;[1 1 1] Apply damage to the destructible mesh
        (Class|DestructibleComponent|ApplyDamage (Variables|Default|GetDestructible) (Variables|Health|GetDamageAmount) (Variables|Default|GetImpactLocation) (* (Variables|Default|GetImpactNormal) -1.0) (* (Variables|Health|GetImpulseStrength) 4e+01))
        ;;[1 1 1] Does debris have collision?
        (if (not (Variables|Setup|GetDebrisHasCollision?))
          ;;[1 1 1] Wait 0.5secs and disable collision
          (Utilities|FlowControl|Delay 0.5)
          (Collision|SetCollisionEnabled (Variables|Default|GetDestructible) "NoCollision"))
        ;[1 1 1] Destroy Actor
        ;;[1 1 1] Destroy the destructible actor?
        (if (Variables|Setup|GetDestroyActor?)
          ;;[1 1 1] Wait DestroyDelay seconds and destroy the actor
          (Utilities|FlowControl|Delay (Variables|Setup|GetDestroyDelay))
          (Actor|DestroyActor))))))

(event Custom|EventMove
  ;[1 1 1] Is movement active?
  (if (Variables|Movement|GetMovementActive?)
    ;[1 1 1] Wait MoveStartDelay seconds
    (Utilities|FlowControl|Delay (Variables|Movement|GetMoveStartDelay))
    (bind _alpha (Timeline|TM_Move PlayFromStart)
      (:Update
        ;[1 1 1] Lerp the actor's location between the start location and end location
        (Transformation|SetActorLocation (Math|Vector|Lerp(Vector) (Variables|Movement|GetStartLocation) (Variables|Movement|GetEndLocation) _alpha) true false)))))

(event Custom|EventSetPlayRate
  ;[1 1 1] Set playrate of the movement TM
  (Components|Timeline|SetPlayRate (Variables|Default|GetTM_Move) (Variables|Movement|GetMovePlayRate)))