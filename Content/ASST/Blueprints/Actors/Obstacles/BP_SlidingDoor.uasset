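; Two-panel sliding door obstacle that opens when an actor tagged Player enters its trigger and closes when it leaves.
; The construction script applies configurable meshes, materials, locations and scales, storing start positions and, until CapturedEndLocation is set, end positions.
; If DoorActive, open and close events wait their delays, then lerp each panel on its own timeline, with closing timelines played in reverse.
; A separate event sets all four timelines' play rate.
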(event OnComponentBeginOverlap(Trigger)
  (params (OverlappedComponent :type Primitive%20Component%20Object%20Reference) (OtherActor :type Actor%20Object%20Reference) (OtherComp :type Primitive%20Component%20Object%20Reference) (OtherBodyIndex :type Integer) (bFromSweep :type Boolean) (SweepResult :type Hit%20Result%20Structure%20%28by%20ref%29))
  ;[1 1 1] Only overlap Player
  (if (Actor|ActorHasTag OtherActor "Player")
    ;[1 1 1] Open doors
    (CallFunction|EventOpen)))

(event OnComponentEndOverlap(Trigger)
  (params (OverlappedComponent :type Primitive%20Component%20Object%20Reference) (OtherActor :type Actor%20Object%20Reference) (OtherComp :type Primitive%20Component%20Object%20Reference) (OtherBodyIndex :type Integer))
  ;[1 1 1] Only overlap Player
  (if (Actor|ActorHasTag OtherActor "Player")
    ;[1 1 1] Close doors
    (CallFunction|EventClose)))

(fn ConstructionScript
  (|CallParentFunction)
  ;[1 1 1] Set Door meshes
  (Components|StaticMesh|SetStaticMesh (Variables|Default|GetMeshL) (Variables|Setup|GetleftMesh))
  (Components|StaticMesh|SetStaticMesh (Variables|Default|GetMeshR) (Variables|Setup|GetRightMesh))
  ;[1 1 1] Set door location
  (Transformation|SetRelativeLocation (Variables|Default|GetMeshL) (Variables|Setup|GetMeshL_Location) false false)
  (Transformation|SetRelativeLocation (Variables|Default|GetMeshR) (Variables|Setup|GetMeshR_Location) false false)
  ;[1 1 1] Set Mesh Materials Index 0
  (Rendering|Material|SetMaterial (Variables|Default|GetMeshL) 0 (Variables|Setup|GetLeftMeshMaterial_0))
  (Rendering|Material|SetMaterial (Variables|Default|GetMeshR) 0 (Variables|Setup|GetRightMeshMaterial_0))
  ;[1 1 1] Set Mesh Materials Index1
  (Rendering|Material|SetMaterial (Variables|Default|GetMeshL) 1 (Variables|Setup|GetLeftMeshMaterial_1))
  (Rendering|Material|SetMaterial (Variables|Default|GetMeshR) 1 (Variables|Setup|GetRightMeshMaterial_1))
  ;[1 1 1] Set mesh scales
  (Transformation|SetWorldScale3D (Variables|Default|GetMeshL) (Variables|Setup|GetMeshLScale))
  (Transformation|SetWorldScale3D (Variables|Default|GetMeshR) (Variables|Setup|GetMeshRScale))
  (Utilities|FlowControl|Sequence
    (:then_0
      ;[1 1 1] LEFT DOOR
      (Utilities|FlowControl|Sequence
        (:then_0
          ;;[1 1 1] Did we capture the end location?, If not save it
          (if (not (Variables|Movement|GetCapturedEndLocation))
            ;;[1 1 1] Capture Final Location for Movement
            (Variables|Movement|SetFinalLocationMeshL (Variables|/Script/Engine.SceneComponent|GetRelativeLocation (Variables|Default|GetMeshL)))))
        (:then_1
          ;;[1 1 1] Set Starting location
          (Variables|Movement|SetOriginalLocationMeshL (Variables|/Script/Engine.SceneComponent|GetRelativeLocation (Variables|Default|GetMeshL))))))
    (:then_1
      ;[1 1 1] RIGHT DOOR
      (Utilities|FlowControl|Sequence
        (:then_0
          ;;[1 1 1] Did we capture the end location? If not, save it
          (if (not (Variables|Movement|GetCapturedEndLocation))
            ;;[1 1 1] Capture Final Location for Movement
            (Variables|Movement|SetFinalLocationMeshR (Variables|/Script/Engine.SceneComponent|GetRelativeLocation (Variables|Default|GetMeshR)))))
        (:then_1
          ;;[1 1 1] Set Starting location
          (Variables|Movement|SetOriginalLocationMeshR (Variables|/Script/Engine.SceneComponent|GetRelativeLocation (Variables|Default|GetMeshR))))))))

(event Custom|EventOpen
  ;[1 1 1] Is the door active?
  (if (Variables|Movement|GetDoorActive?)
    ;[1 1 1] Wait OpenDelay seconds
    (Utilities|FlowControl|Delay (Variables|Movement|GetOpenDelay))
    (Utilities|FlowControl|Sequence
      (:then_0
        ;[1 1 1] Lerp the position of the Left Door
        (bind _alpha (Timeline|TM_Open_Left PlayFromStart)
          (:Update
            (Transformation|SetRelativeLocation (Variables|Default|GetMeshL) (Math|Vector|Lerp(Vector) (Variables|Movement|GetOriginalLocationMeshL) (Variables|Movement|GetFinalLocationMeshL) _alpha) false true))))
      (:then_1
        ;[1 1 1] Lerp the position of the Right Door
        (bind _alpha_2 (Timeline|TM_Open_Right PlayFromStart)
          (:Update
            (Transformation|SetRelativeLocation (Variables|Default|GetMeshR) (Math|Vector|Lerp(Vector) (Variables|Movement|GetOriginalLocationMeshR) (Variables|Movement|GetFinalLocationMeshR) _alpha_2) false true)))))))

(event Custom|EventClose
  ;[1 1 1] Is the door active?
  (if (Variables|Movement|GetDoorActive?)
    ;[1 1 1] Wait CloseDelay seconds
    (Utilities|FlowControl|Delay (Variables|Movement|GetCloseDelay))
    (Utilities|FlowControl|Sequence
      (:then_0
        ;[1 1 1] Lerp the position of the Left Door
        (bind _alpha (Timeline|TM_Close_Left ReverseFromEnd)
          (:Update
            (Transformation|SetRelativeLocation (Variables|Default|GetMeshL) (Math|Vector|Lerp(Vector) (Variables|Movement|GetOriginalLocationMeshL) (Variables|Movement|GetFinalLocationMeshL) _alpha) false true))))
      (:then_1
        ;[1 1 1] Lerp the position of the Right Door
        (bind _alpha_2 (Timeline|TM_Close_Right ReverseFromEnd)
          (:Update
            (Transformation|SetRelativeLocation (Variables|Default|GetMeshR) (Math|Vector|Lerp(Vector) (Variables|Movement|GetOriginalLocationMeshR) (Variables|Movement|GetFinalLocationMeshR) _alpha_2) false true)))))))

(event Custom|EventSetPlayRate
  ;[1 1 1] Set the playrate for all the timelines
  (Components|Timeline|SetPlayRate (Variables|Default|GetTM_Open_Right) (Variables|Movement|GetPlayRate)))