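; BP_PointsCache is a destructible points pickup that can shuttle between two locations and rewards the player ship when destroyed.
; Forward and backward timelines call each other to lerp the actor back and forth, with configurable delays and play rates.
; The construction script records the start location, and also the end location while CaptureEndLocation is off.
; Hit counts up to HitsUntilDeath, then spawns an explosion, adds points to BP_PlayerShip, plays a sound and destroys the actor.
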(event EventBeginPlay
  ;[1 1 1] Save starting location
  (Variables|Movement|SetStartLocation (Transformation|GetActorLocation))
  ;[1 1 1] Set PlayRate and Start Movement
  (CallFunction|EventSetPlayRate)
  (CallFunction|EventForward))

(fn ConstructionScript
  (bind _returnvalue (Transformation|GetActorLocation))
  (Rendering|Material|SetMaterial (Variables|Default|GetMesh) 0 (Variables|Setup|GetMaterial))
  (Utilities|FlowControl|Sequence
    (:then_0
      (if (not (Variables|Movement|GetCaptureEndLocation))
        ;[1 1 1] Capture Final Location for Movement
        (Variables|Movement|SetEndLocation _returnvalue)))
    (:then_1
      ;[1 1 1] Set Starting location
      (Variables|Movement|SetStartLocation _returnvalue))))

(event Custom|EventForward
  ;[1 1 1] Is Movement Active?
  (if (Variables|Movement|GetMovementActive?)
    ;[1 1 1] Delay Movement by specified amount
    (Utilities|FlowControl|Delay (Variables|Movement|GetMovementStartDelay))
    ;[1 1 1] Move obstacle to location - TM is 2secs
    (bind _alpha (Timeline|TM_Forward PlayFromStart)
      (:Update
        (Transformation|SetActorLocation (Math|Vector|Lerp(Vector) (Variables|Movement|GetStartLocation) (Variables|Movement|GetEndLocation) _alpha) false false))
      (:Finished
        ;[1 1 1] Once movement is complete - start going back
        (CallFunction|EventBackwards)))))

(event Custom|EventBackwards
  ;[1 1 1] Is movement active?
  (if (Variables|Movement|GetMovementActive?)
    ;[1 1 1] Wait for the specified time before moving
    (Utilities|FlowControl|Delay (Variables|Movement|GetMovementBackDelay))
    ;[1 1 1] Move obstacle to location - TM is 2secs
    (bind _alpha (Timeline|TM_Backwards ReverseFromEnd)
      (:Update
        (Transformation|SetActorLocation (Math|Vector|Lerp(Vector) (Variables|Movement|GetStartLocation) (Variables|Movement|GetEndLocation) _alpha) false false))
      (:Finished
        ;[1 1 1] When movement is finished, go forward
        (CallFunction|EventForward)))))

(event Custom|EventSetPlayRate
  ;[1 1 1] Set the PlayRate for the Forward TM
  (Components|Timeline|SetPlayRate (Variables|Default|GetTM_Forward) (Variables|Movement|GetForwardPlayRate))
  ;[1 1 1] Set the PlayRate for the Backwards TM
  (Components|Timeline|SetPlayRate (Variables|Default|GetTM_Backwards) (Variables|Movement|GetBackwardsPlayRate)))

(event Collision|EventHit
  (params (MyComp :type Primitive%20Component%20Object%20Reference) (Other :type Actor%20Object%20Reference) (OtherComp :type Primitive%20Component%20Object%20Reference) (bSelfMoved :type Boolean) (HitLocation :type Vector :default "0, 0, 0") (HitNormal :type Vector :default "0, 0, 0") (NormalImpulse :type Vector :default "0, 0, 0") (Hit :type Hit%20Result%20Structure%20%28by%20ref%29))
  ;[1 1 1] Check to see if the number of hits is bigger than HitsUntilDeath
  (if (>= (Variables|Setup|GetHitCounter) (Variables|Setup|GetHitsUntilDeath))
    ;[1 1 1] Spawn fire effect
    (bind _returnvalue (Effects|SpawnEmitteratLocation (Variables|Setup|GetExplosionParticles) (Transformation|GetActorLocation) :!label _label))
    (Utilities|IsValid _returnvalue
      (:Is%20Valid
        ;[1 1 1] Scale the effect
        (Transformation|SetWorldScale3D _returnvalue "5.000000,5.000000,5.000000"))
      (:Is%20Not%20Valid
        _))
    ;[1 1 1] Cast to Player and add points by the specificed amount
    (bind _asbp_player_ship (Utilities|Casting|CastToBP_PlayerShip (Game|Player|GetPlayerPawn 0)))
    (Default|FnAddPoints _asbp_player_ship (Variables|Setup|GetPointsToAdd))
    ;[1 1 1] Play the sound fx
    (Audio|PlaySound2D (Variables|Setup|GetSound))
    ;[1 1 1] Destroy the actor
    (Actor|DestroyActor)
    (else
      ;[1 1 1] Add 1 to hit counter
      (Variables|Setup|SetHitCounter (+ (Variables|Setup|GetHitCounter) 1))
      ;[1 1 1] Check counter again
      (if (>= (Variables|Setup|GetHitCounter) (Variables|Setup|GetHitsUntilDeath))
        (goto _label)))))