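; Bomb pickup actor that adds bombs to the player ship when the player touches it.
; On overlap it halves its scale for visibility, then either sticks to the player, optionally rotating, or gets picked up immediately.
; Pickup passes NumberOfBombs to BP_PlayerShip, plays a 2D sound and destroys the actor.
; The sticking and rotation events are defined outside this graph, and construction copies Shrink into ShrinkPickUp.
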(event OnComponentBeginOverlap(Trigger)
  (params (OverlappedComponent :type Primitive%20Component%20Object%20Reference) (OtherActor :type Actor%20Object%20Reference) (OtherComp :type Primitive%20Component%20Object%20Reference) (OtherBodyIndex :type Integer) (bFromSweep :type Boolean) (SweepResult :type Hit%20Result%20Structure%20%28by%20ref%29))
  ;[1 1 1] Overlap only the Player
  (if (Actor|ActorHasTag OtherActor "Player")
    ;[1 1 1] When picked up set scale to half size to allow more visibility
    (Transformation|SetActorScale3D "0.500000,0.500000,0.500000")
    (if (Variables|Setup|GetStickToPlayer?)
      (if (Variables|Setup|GetRotateWhileSticking?)
        (CallFunction|EventRotateWhileSticking))
      (CallFunction|EventSticktoPlayer)
      (else
        (CallFunction|EventPickedUp)))))

(event EventEventPickedUp
  ;[1 1 1] Cast to Player and add bombs based on NumberOfBombs
  (bind _asbp_player_ship (Utilities|Casting|CastToBP_PlayerShip (Game|Player|GetPlayerPawn 0)))
  (Default|FnAddBombs _asbp_player_ship (Variables|Setup|GetNumberOfBombs))
  ;[1 1 1] Play sound fx
  (Audio|PlaySound2D (Variables|Setup|GetSound))
  ;[1 1 1] Destroy actor
  (Actor|DestroyActor))

(fn ConstructionScript
  ;[1 1 1] Set default value of Shrink
  (Variables|Default|SetShrinkPickUp? (Variables|Setup|GetShrink?)))