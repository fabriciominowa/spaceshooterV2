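; Checkpoint pickup actor that records the player ship's progress when flown through.
; On trigger overlap by a living, Player-tagged BP_PlayerShip, it passes itself, track state and music settings to the ship's FnSaveCheckPoint, then plays a 2D sound.
; The ring mesh spins from BeginPlay through a short looping timer that the rotation event re-sets on every call, rather than using Tick.
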(event OnComponentBeginOverlap(Trigger)
  (params (OverlappedComponent :type Primitive%20Component%20Object%20Reference) (OtherActor :type Actor%20Object%20Reference) (OtherComp :type Primitive%20Component%20Object%20Reference) (OtherBodyIndex :type Integer) (bFromSweep :type Boolean) (SweepResult :type Hit%20Result%20Structure%20%28by%20ref%29))
  ;[1 1 1] Only overlap Player
  (if (Actor|ActorHasTag OtherActor "Player")
    (bind _asbp_player_ship (Utilities|Casting|CastToBP_PlayerShip OtherActor))
    ;[1 1 1] Only save is Player is NOT dead
    (if (not (Variables|/Game/ASST/Blueprints/Characters/Player/BP_PlayerShip.BP_PlayerShip_C|GetIsDead _asbp_player_ship))
      ;[1 1 1] Save Checkpoint data
      (Default|FnSaveCheckPoint _asbp_player_ship self (Variables|Setup|GetCurrentTrack) (Variables|Setup|GetBackgroundMusic) (Variables|Setup|GetMusicID) (Variables|Setup|GetMusic%20Multiplier) (Variables|Setup|GetOnTrack?))
      ;[1 1 1] Play sound fx
      (Audio|PlaySound2D (Variables|Setup|GetSoundFX)))))

(event Custom|EventRotateRing
  (Utilities|Time|SetTimerbyEvent (delegate Custom|EventRotateRing) 0.01 true)
  ;[1 1 1] Add rotation to the mesh
  (Transformation|AddLocalRotation (Variables|Default|GetMesh) "0, 0,-1.000000" false false))

(event EventBeginPlay
  ;[1 1 1] Rotate the ring
  (CallFunction|EventRotateRing))

(fn ConstructionScript)