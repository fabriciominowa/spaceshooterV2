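; BP_PickUpBase is the base pickup actor, able to travel to the player ship and stick to it.
; On BeginPlay, All-Range and Track mode flags gate timeline movement, either lerping onto the player or stepping toward them by look-at direction.
; A one-shot stick event makes Tick follow the player, waits, optionally shrinks the pickup, then fires EventPickedUp for child overrides.
; A separate looping timer event spins it around local X.
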(event Custom|EventPickedUp
  ;[1 1 1] CUSTOM EVENTS
)

(event EventBeginPlay
  ;[1 1 1] Save Player reference
  (Variables|Default|SetPlayerRef (Game|Player|GetPlayerPawn 0))
  ;[1 1 1] Move towards Player while in All-Range Mode?
  (if (Variables|Setup|GetMoveToPlayerARM?)
    (CallFunction|EventMovetoPlayer true false)
    (else
      ;[1 1 1] Move towards Player while in Track Mode?
      (if (Variables|Setup|GetMoveToPlayerTrackMode?)
        (CallFunction|EventMovetoPlayer false true)))))

(event EventTick
  (params (DeltaSeconds :type Float%20%28single-precision%29))
  (bind _playerref (Variables|Default|GetPlayerRef))
  (bind _returnvalue (Transformation|GetActorRotation _playerref))
  (if (Variables|Setup|GetSticking?)
    ;[1 1 1] Set the PickUps location and rotation to the Player's
    (Transformation|SetActorLocationAndRotation (Transformation|GetActorLocation _playerref) (Math|Rotator|MakeRotator (.roll (Transformation|GetActorRotation)) (.pitch _returnvalue) (.yaw _returnvalue)) false true)))

(fn ConstructionScript)

(event Custom|EventRotateWhileSticking
  (Utilities|Time|SetTimerbyEvent (delegate Custom|EventRotateWhileSticking) 0.02 true)
  ;[1 1 1] Rotate Pickup on its X axis while sticking to Player
  (Transformation|AddActorLocalRotation (Math|Rotator|MakeRotator (Variables|Setup|GetStickingRotationRate) 0.0 0.0) false true))

(event Custom|EventMoveToPlayer
  (params (MoveARM? :type Boolean) (MoveTrack? :type Boolean))
  ;[1 1 1] Determine whether TrackMode is active from Player
  (bind _asbp_player_ship (Utilities|Casting|CastToBP_PlayerShip (Variables|Default|GetPlayerRef)))
  (if (Variables|/Game/ASST/Blueprints/Characters/Player/BP_PlayerShip.BP_PlayerShip_C|GetTrackModeActive _asbp_player_ship)
    (if MoveARM?
      ;[1 1 1] Determine which PickUpMoveMode to use
      (switch Utilities|FlowControl|Switch|SwitchonEnum_PickUpMoveMode (Variables|Default|GetMoveMode) :!label _label
        (:NewEnumerator0
          ;[1 1 1] Always reach Player
          (bind _alpha (Timeline|TM_ReachPlayer Play)
            (:Update
              (Transformation|SetActorLocation (Math|Vector|Lerp(Vector) (Transformation|GetActorLocation) (Transformation|GetActorLocation (Variables|Default|GetPlayerRef)) _alpha) false true))))
        (:NewEnumerator1
          ;[1 1 1] Move Towards Player
          (Timeline|TM_MoveToPlayer Play
            (:Update
              (Transformation|AddActorWorldOffset (* (Math|Vector|GetForwardVector (Math|Rotator|FindLookatRotation (Transformation|GetActorLocation) (Transformation|GetActorLocation (Variables|Default|GetPlayerRef)))) (Variables|Setup|GetSpeed)) false true))))))
    (elif MoveTrack?
      (goto _label))))

(event Custom|EventStickToPlayer
  (Utilities|FlowControl|DoOnce false
    (:Completed
      ;[1 1 1] Get PickUp to stick to Player
      (Variables|Setup|SetSticking? true)
      (Utilities|FlowControl|Delay (Variables|Setup|GetTimeToStick))
      (if (Variables|Setup|GetShrinkPickUp?)
        ;[1 1 1] Shrink the PickUp from its current scale to 0 in 2 seconds
        (bind _alpha (Timeline|TM_Shrink Play)
          (:Update
            (Transformation|SetActorScale3D (Math|Vector|Lerp(Vector) (Transformation|GetActorScale3D) "0.070000,0.070000,0.070000" _alpha)))
          (:Finished
            ;[1 1 1] Dummy Event that can be overriden on the child class
            (CallFunction|EventPickedUp :!label _label)))
        (else
          (goto _label))))))