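; BP_Bomb is a projectile bomb that explodes on a timer and deals radial damage.
; Its construction script sets the projectile movement velocity and actor tags from variables.
; On BeginPlay the mesh ignores the player pawn when moving, then a travel-time delay triggers the explosion.
; The explosion applies full damage within the radius, spawns a scaled-up particle effect, plays sound and camera shake, then destroys the actor after a brief delay.
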(event Custom|EventExplode
  (bind _mesh (Variables|Default|GetMesh))
  (bind _returnvalue (Transformation|GetWorldLocation _mesh))
  ;[1 1 1] Apply radial damage
  (Game|Damage|ApplyRadialDamage (Variables|Setup|GetBaseDamage) (Transformation|GetWorldLocation (Variables|Default|GetMesh)) (Variables|Setup|GetDamageRadius) 0 0 self 0 true "ECC_Visibility")
  ;[1 1 1] Spawn and scale the explosion emitter
  (bind _returnvalue_2 (Effects|SpawnEmitteratLocation (Variables|Setup|GetExplosionParticle) _returnvalue))
  (Utilities|IsValid _returnvalue_2
    (:Is%20Valid
      (Transformation|SetWorldScale3D _returnvalue_2 "40.000000,40.000000,40.000000"))
    (:Is%20Not%20Valid
      _))
  ;[1 1 1] Play explosion sound
  (Audio|PlaySoundatLocation (Variables|Setup|GetExplosionSound) _returnvalue)
  ;[1 1 1] Shake camera
  (Camera|PlayWorldCameraShake "/Game/ASST/Blueprints/Actors/Crash/BP_CameraShake.BP_CameraShake_C" (Transformation|GetActorLocation) 0.0 1.5e+04)
  ;[1 1 1] Wait for 0.2secs and destroy the actor
  (Utilities|FlowControl|Delay 0.2)
  (Actor|DestroyActor))

(event EventBeginPlay
  ;[1 1 1] Ignore Player Pawn
  (Collision|IgnoreActorwhenMoving (Variables|Default|GetMesh) (Game|Player|GetPlayerPawn 0) true)
  ;[1 1 1] Wait TravelTime seconds before exploding and doing damage
  (Utilities|FlowControl|Delay (Variables|Setup|GetTravelTime))
  ;[1 1 1] Explode
  (CallFunction|EventExplode))

(fn ConstructionScript
  ;[1 1 1] Ser velocity
  (Variables|/Script/Engine.MovementComponent|SetVelocity (Variables|Default|GetProjectileMovement) (Variables|Setup|GetProjectileVelocity))
  ;[1 1 1] Set actor tags
  (Variables|Default|SetTags (Variables|Default|GetActorTags)))