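; Enemy laser projectile that flies at a configurable velocity and expires after a set lifetime.
; The construction script applies velocity and actor tags; a mesh hit spawns explosion particles and sound, then destroys the actor after a short delay, with no damage applied here.
; An optional never-miss mode stores a target and uses a fast looping timer, re-armed on each call, to continually re-aim rotation and velocity at it.
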(event OnComponentHit(LaserMesh)
  (params (HitComponent :type Primitive%20Component%20Object%20Reference) (OtherActor :type Actor%20Object%20Reference) (OtherComp :type Primitive%20Component%20Object%20Reference) (NormalImpulse :type Vector :default "0, 0, 0") (Hit :type Hit%20Result%20Structure%20%28by%20ref%29))
  (bind _returnvalue (Transformation|GetWorldLocation HitComponent))
  ;[1 1 1] Spawn emitter at impact location
  (Effects|SpawnEmitteratLocation (Variables|Setup|GetExplosionParticles) _returnvalue)
  ;[1 1 1] Play explosion sound
  (Audio|PlaySoundatLocation (Variables|Setup|GetExplosionSound) _returnvalue)
  ;[1 1 1] Wait 0.2secs and destroy the actor
  (Utilities|FlowControl|Delay 0.2)
  (Actor|DestroyActor))

(event Custom|EventNeverMiss
  (params (TargetActor :type Actor%20Object%20Reference))
  ;[1 1 1] Set TargetActor and call EventNeverMissTimer
  (Variables|Setup|SetTargetActor TargetActor)
  (CallFunction|EventNeverMissTimer))

(event Custom|EventNeverMissTimer
  (bind _returnvalue (Transformation|GetActorLocation))
  (bind _targetactor (Variables|Setup|GetTargetActor))
  (bind _returnvalue_2 (Transformation|GetActorLocation _targetactor))
  (bind _returnvalue_3 (Math|Rotator|FindLookatRotation _returnvalue _returnvalue_2))
  (Utilities|Time|SetTimerbyEvent (delegate Custom|EventNeverMissTimer) 0.01 true)
  ;[1 1 1] Set rotation towards player
  (Transformation|SetActorRotation _returnvalue_3)
  ;[1 1 1] Set velocity towards player
  (Variables|/Script/Engine.MovementComponent|SetVelocity (Variables|Default|GetProjectileMovement) (* (Math|Vector|GetForwardVector _returnvalue_3) (Variables|Setup|GetNeverMissSpeed))))

(event EventBeginPlay
  ;[1 1 1] Set Laser lifespan
  (Actor|SetLifeSpan (Variables|Setup|GetTimeToLive)))

(fn ConstructionScript
  ;[1 1 1] Set velocity
  (Variables|/Script/Engine.MovementComponent|SetVelocity (Variables|Default|GetProjectileMovement) (Variables|Setup|GetProjectileVelocity))
  ;[1 1 1] Set actor tags
  (Variables|Default|SetTags (Variables|Default|GetActorTags)))