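; BP_Mine is an enemy mine that explodes when an actor tagged Player overlaps its collision sphere.
; It sets its own tags from the DamageType setting, then applies full radial damage with itself as causer, so the tag can identify the kind of hit.
; It spawns a scaled explosion effect and sound at the mesh, then destroys itself after a short delay.
; The construction script sizes the trigger sphere from CollisionRadius.
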(event OnComponentBeginOverlap(Collision)
  (params (OverlappedComponent :type Primitive%20Component%20Object%20Reference) (OtherActor :type Actor%20Object%20Reference) (OtherComp :type Primitive%20Component%20Object%20Reference) (OtherBodyIndex :type Integer) (bFromSweep :type Boolean) (SweepResult :type Hit%20Result%20Structure%20%28by%20ref%29))
  (bind _mesh (Variables|Default|GetMesh))
  (bind _returnvalue (Transformation|GetWorldLocation _mesh))
  ;[1 1 1] Check to see if Player overlapped
  (if (Actor|ActorHasTag OtherActor "Player")
    ;[1 1 1] Set damage type
    (switch Utilities|FlowControl|Switch|SwitchonEnum_DamageType (Variables|Setup|GetDamageType)
      (:NewEnumerator0
        (Variables|Default|SetTags (Variables|Default|GetCrashTag)))
      (:NewEnumerator1
        (Variables|Default|SetTags (Variables|Default|GetLightTag)))
      (:NewEnumerator2
        (Variables|Default|SetTags (Variables|Default|GetHeavyTag)))
      (:NewEnumerator3
        (Variables|Default|SetTags (Variables|Default|GetShieldBreakTag)))
      (:NewEnumerator4
        (Variables|Default|SetTags (Variables|Default|GetInstaDeathTag))))
    ;[1 1 1] Apply radial damage
    (Game|Damage|ApplyRadialDamage 1.0 (Transformation|GetActorLocation) (Variables|Setup|GetDamageRadius) 0 0 self 0 true "ECC_Visibility")
    ;[1 1 1] Spawn emitter at impact location and scale it
    (bind _returnvalue_2 (Effects|SpawnEmitteratLocation (Variables|Setup|GetExplosionParticles) _returnvalue))
    (Utilities|IsValid _returnvalue_2
      (:Is%20Valid
        (Transformation|SetWorldScale3D _returnvalue_2 "40.000000,40.000000,40.000000"))
      (:Is%20Not%20Valid
        _))
    ;[1 1 1] Play explosion sound
    (Audio|PlaySoundatLocation (Variables|Setup|GetExplosionSound) _returnvalue)
    ;[1 1 1] Wait for 0.2secs and destroy the actor
    (Utilities|FlowControl|Delay 0.2)
    (Actor|DestroyActor)))

(fn ConstructionScript
  ;[1 1 1] Set the collision radius
  (Components|Sphere|SetSphereRadius (Variables|Default|GetCollision) (Variables|Setup|GetCollisionRadius) true))