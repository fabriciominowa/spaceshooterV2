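; Homing projectile actor that explodes on hit, dealing full radial damage with particles and sound, then destroys itself after a short delay.
; EventFollowTarget receives a target and enables ProjectileMovement homing on its root component.
; With NeverMisses set, a fast looping timer also snaps rotation and velocity toward the followed target at NeverMissSpeed.
; It ignores the player pawn, has a limited lifespan, and takes initial velocity and tags from variables.
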(event OnComponentHit(Sphere)
  (params (HitComponent :type Primitive%20Component%20Object%20Reference) (OtherActor :type Actor%20Object%20Reference) (OtherComp :type Primitive%20Component%20Object%20Reference) (NormalImpulse :type Vector :default "0, 0, 0") (Hit :type Hit%20Result%20Structure%20%28by%20ref%29))
  (bind _returnvalue (Transformation|GetWorldLocation HitComponent))
  ;[1 1 1] Hit Something
  ;;[1 1 1] Apply radial damage
  (Game|Damage|ApplyRadialDamage (Variables|Setup|GetBaseDamage) (Transformation|GetWorldLocation HitComponent) (Variables|Setup|GetDamageRadius) 0 0 self 0 true "ECC_Visibility")
  ;;[1 1 1] Spawn emitter at impact location
  (Effects|SpawnEmitteratLocation (Variables|Setup|GetExplosionParticles) _returnvalue)
  ;;[1 1 1] Play explosion sound
  (Audio|PlaySoundatLocation (Variables|Setup|GetExplosionSound) _returnvalue)
  ;;[1 1 1] Wait for 0.2secs and destroy the actor
  (Utilities|FlowControl|Delay 0.2)
  (Actor|DestroyActor))

(event Custom|EventFollowTarget
  (params (ActorToFollow :type Actor%20Object%20Reference))
  (bind _projectilemovement (Variables|Default|GetProjectileMovement))
  ;[1 1 1] Follow target
  ;;[1 1 1] Make sure actor is valid
  (if (Utilities|IsValid ActorToFollow)
    ;;[1 1 1] Set projectile to Homing and pass the correct parameters
    (Variables|/Script/Engine.ProjectileMovementComponent|SetbIsHomingProjectile (Variables|Default|GetProjectileMovement) true)
    (bind _output_get (Variables|Default|SetTargetActor ActorToFollow))
    (Variables|/Script/Engine.ProjectileMovementComponent|SetHomingTargetComponent _projectilemovement (VehicleSound|GetRootComponent _output_get))
    (Variables|/Script/Engine.ProjectileMovementComponent|SetHomingAccelerationMagnitude _projectilemovement 4e+04)
    (Variables|Default|SetFollowingTarget? true)))

(event Custom|EventNeverMissTimer
  (bind _returnvalue (Transformation|GetActorLocation))
  (bind _targetactor (Variables|Default|GetTargetActor))
  (bind _returnvalue_2 (Transformation|GetActorLocation _targetactor))
  (bind _returnvalue_3 (Math|Rotator|FindLookatRotation _returnvalue _returnvalue_2))
  ;[1 1 1] Event NeverMiss - projectile NEVER misses the target
  (Utilities|Time|SetTimerbyEvent (delegate Custom|EventNeverMissTimer) 0.01 true)
  ;;[1 1 1] Check if you are following the target
  (if (Variables|Default|GetFollowingTarget?)
    ;;[1 1 1] Set the actor rotation towards the target
    (Transformation|SetActorRotation _returnvalue_3)
    ;;[1 1 1] Set the velocity vector
    (Variables|/Script/Engine.MovementComponent|SetVelocity (Variables|Default|GetProjectileMovement) (* (Math|Vector|GetForwardVector _returnvalue_3) (Variables|Default|GetNeverMissSpeed)))))

(event EventBeginPlay
  ;[1 1 1] Set Fireball lifespan
  (Actor|SetLifeSpan (Variables|Default|GetTimeToLive))
  ;[1 1 1] Is the projectile a NeverMiss?
  (if (Variables|Default|GetNeverMisses)
    ;[1 1 1] Start tick timer
    (CallFunction|EventNeverMissTimer))
  ;[1 1 1] Ignore Player Pawn
  (Collision|IgnoreActorwhenMoving (Variables|Default|GetSphere) (Game|Player|GetPlayerPawn 0) true))

(fn ConstructionScript
  ;[1 1 1] Set velocity
  (Variables|/Script/Engine.MovementComponent|SetVelocity (Variables|Default|GetProjectileMovement) (Variables|Setup|GetProjectileVelocity))
  ;[1 1 1] Set actor tags
  (Variables|Default|SetTags (Variables|Default|GetActorTags)))