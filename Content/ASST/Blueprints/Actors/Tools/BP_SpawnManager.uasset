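; Spawn manager actor that activates every BP_EnemySpawner in the level carrying its SpawnerTag.
; SpawnMethod selects either spawning on BeginPlay or arming box and sphere triggers, each firing once when a Player-tagged actor overlaps.
; Tagged spawners spawn a single enemy, or receive count and frequency settings to spawn one immediately and the rest through their multiple-spawn event.
; The construction script sets trigger visibility and sphere radius.
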(event OnComponentBeginOverlap(TriggerBox)
  (params (OverlappedComponent :type Primitive%20Component%20Object%20Reference) (OtherActor :type Actor%20Object%20Reference) (OtherComp :type Primitive%20Component%20Object%20Reference) (OtherBodyIndex :type Integer) (bFromSweep :type Boolean) (SweepResult :type Hit%20Result%20Structure%20%28by%20ref%29))
  ;[1 1 1] Check if Player overlapped trigger, if so call EventPlayerDetected
  (if (and (Actor|ActorHasTag OtherActor "Player") (Variables|Default|GetUseTriggers))
    (Utilities|FlowControl|DoOnce false
      (:Completed
        (CallFunction|EventCallSpawners)))))

(event OnComponentBeginOverlap(TriggerSphere)
  (params (OverlappedComponent :type Primitive%20Component%20Object%20Reference) (OtherActor :type Actor%20Object%20Reference) (OtherComp :type Primitive%20Component%20Object%20Reference) (OtherBodyIndex :type Integer) (bFromSweep :type Boolean) (SweepResult :type Hit%20Result%20Structure%20%28by%20ref%29))
  ;[1 1 1] Check if Player overlapped trigger, if so call EventPlayerDetected
  (if (and (Actor|ActorHasTag OtherActor "Player") (Variables|Default|GetUseTriggers))
    (Utilities|FlowControl|DoOnce false
      (:Completed
        (CallFunction|EventCallSpawners)))))

(event EventBeginPlay
  ;[1 1 1] Select spawn method
  (switch Utilities|FlowControl|Switch|SwitchonEnum_EnemySpawnMethod (Variables|Setup-General|GetSpawnMethod)
    (:NewEnumerator0
      (CallFunction|EventCallSpawners))
    (:NewEnumerator2
      (Variables|Default|SetUseTriggers true))))

(fn ConstructionScript
  (Rendering|SetVisibility (Variables|Default|GetTriggerBox) (Variables|Setup-General|GetShowTrigger?) false)
  (Components|Sphere|SetSphereRadius (Variables|Default|GetTriggerSphere) (Variables|Setup-General|GetSphereTriggerRadius) true))

(event Custom|EventCallSpawners
  ;[1 1 1] Check all Enemy Spawners in the level
  (bind _outactors (Actor|GetAllActorsOfClass "/Game/ASST/Blueprints/Actors/Tools/BP_EnemySpawner.BP_EnemySpawner_C"))
  (for _array_element _outactors
    ;[1 1 1] Check if they have the specified tag
    (if (Actor|ActorHasTag _array_element (Variables|Setup-General|GetSpawnerTag))
      ;[1 1 1] Spawn multiple enemies?
      (if (Variables|Setup-MultipleEnemies|GetSpawnMultipleEnemies?)
        ;[1 1 1] Set all parameters needed to spawn multiple enemies
        (Variables|/Game/ASST/Blueprints/Actors/Tools/BP_EnemySpawner.BP_EnemySpawner_C|SetSpawnNumber _array_element (Variables|Setup-MultipleEnemies|GetSpawnNumber))
        (Variables|/Game/ASST/Blueprints/Actors/Tools/BP_EnemySpawner.BP_EnemySpawner_C|SetSpawnFrequency _array_element (Variables|Setup-MultipleEnemies|GetSpawnFrequency))
        (Variables|/Game/ASST/Blueprints/Actors/Tools/BP_EnemySpawner.BP_EnemySpawner_C|SetSpawnCount _array_element 1)
        ;[1 1 1] Spawn enemy immediately and call EventMultiple Spawn to spawn the rest
        (Default|EventSpawnEnemy _array_element)
        (Default|EventMultipleSpawn _array_element)
        (else
          ;[1 1 1] Spawn single enemy
          (Default|EventSpawnEnemy _array_element))))))