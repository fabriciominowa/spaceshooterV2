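; Spline-based tool actor that builds modular corridors and chains them through end joints.
; The construction script lays a two-material spline mesh along each segment, labels points with game-hidden index text, and optionally places an end mesh chosen by JointType (left, right, closed, T or Y).
; The SpawnConnection event, gated by a flag, spawns another BP_CorridorBuilder at the joint's connector, with yaw offset from the spline end to match the chosen branch.
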(event Custom|Spawn%20Connection
  (bind _spline (Variables|Default|GetSpline))
  (bind _spline_2 (Variables|Default|GetSpline))
  (bind _spline_3 (Variables|Default|GetSpline))
  (bind _spline_4 (Variables|Default|GetSpline))
  (bind _spline_5 (Variables|Default|GetSpline))
  (bind _spline_6 (Variables|Default|GetSpline))
  (bind _returnvalue (Spline|GetNumberOfSplinePoints _spline_6))
  (bind _returnvalue_2 (Spline|GetNumberOfSplinePoints _spline))
  (bind _returnvalue_3 (Spline|GetNumberOfSplinePoints _spline_2))
  (bind _returnvalue_4 (Spline|GetNumberOfSplinePoints _spline_3))
  (bind _returnvalue_5 (Spline|GetNumberOfSplinePoints _spline_4))
  (bind _returnvalue_6 (Spline|GetNumberOfSplinePoints _spline_5))
  (bind _returnvalue_7 (Spline|GetRotationatSplinePoint _spline_6 _returnvalue "World"))
  (bind _returnvalue_8 (Spline|GetRotationatSplinePoint _spline _returnvalue_2 "World"))
  (bind _returnvalue_9 (Spline|GetRotationatSplinePoint _spline_2 _returnvalue_3 "World"))
  (bind _returnvalue_10 (Spline|GetRotationatSplinePoint _spline_3 _returnvalue_4 "World"))
  (bind _returnvalue_11 (Spline|GetRotationatSplinePoint _spline_4 _returnvalue_5 "World"))
  (bind _returnvalue_12 (Spline|GetRotationatSplinePoint _spline_5 _returnvalue_6 "World"))
  ;[1 1 1] Check if you are allowed to spawn a connection
  (if (Variables|Setup-Connection|GetSpawnConnection?)
    ;[1 1 1] Choose joint type to spawn
    (switch Utilities|FlowControl|Switch|SwitchonEnum_CorridorJointType (Variables|Setup-General|GetJointType)
      (:NewEnumerator0
        ;[1 1 1] Get Left location
        (Variables|Setup-Connection|SetSpawnVector (Transformation|GetWorldLocation (Variables|Default|GetConnectJointLeft)))
        ;[1 1 1] Get rotation
        (Variables|Setup-Connection|SetSpawnRotation (Math|Rotator|MakeRotator (.roll _returnvalue_8) (.pitch (Transformation|GetActorRotation)) (- (.yaw _returnvalue_8) 9e+01))))
      (:NewEnumerator1
        ;[1 1 1] Get Right location
        (Variables|Setup-Connection|SetSpawnVector (Transformation|GetWorldLocation (Variables|Default|GetConnectJointRight)))
        ;[1 1 1] Get rotation
        (Variables|Setup-Connection|SetSpawnRotation (Math|Rotator|MakeRotator (.roll _returnvalue_9) (.pitch (Transformation|GetActorRotation)) (+ (.yaw _returnvalue_9) 9e+01))))
      (:NewEnumerator3
        ;[1 1 1] Get T Joint Location
        (switch Utilities|FlowControl|Switch|SwitchonEnum_Corridor_SpawnPlace (Variables|Setup-Connection|GetSpawnLocation)
          (:NewEnumerator0
            (Variables|Setup-Connection|SetSpawnVector (Transformation|GetWorldLocation (Variables|Default|GetConnectJointLeft)))
            ;[1 1 1] Get rotation
            (Variables|Setup-Connection|SetSpawnRotation (Math|Rotator|MakeRotator (.roll _returnvalue_10) (.pitch _returnvalue_10) (- (.yaw _returnvalue_10) 9e+01))))
          (:NewEnumerator1
            (Variables|Setup-Connection|SetSpawnVector (Transformation|GetWorldLocation (Variables|Default|GetConnectJointRight)))
            ;[1 1 1] Get rotation
            (Variables|Setup-Connection|SetSpawnRotation (Math|Rotator|MakeRotator (.roll _returnvalue_11) (.pitch _returnvalue_11) (+ (.yaw _returnvalue_11) 9e+01))))))
      (:NewEnumerator4
        ;[1 1 1] Get Y Joint Location
        (switch Utilities|FlowControl|Switch|SwitchonEnum_Corridor_SpawnPlace (Variables|Setup-Connection|GetSpawnLocation)
          (:NewEnumerator0
            (Variables|Setup-Connection|SetSpawnVector (Transformation|GetWorldLocation (Variables|Default|GetConnectJointY_Left)))
            ;[1 1 1] Get rotation
            (Variables|Setup-Connection|SetSpawnRotation (Math|Rotator|MakeRotator (.roll _returnvalue_12) (.pitch _returnvalue_12) (- (.yaw _returnvalue_12) 45.0))))
          (:NewEnumerator1
            (Variables|Setup-Connection|SetSpawnVector (Transformation|GetWorldLocation (Variables|Default|GetConnectJointY_Right)))
            ;[1 1 1] Get rotation
            (Variables|Setup-Connection|SetSpawnRotation (Math|Rotator|MakeRotator (.roll _returnvalue_7) (.pitch _returnvalue_7) (+ (.yaw _returnvalue_7) 45.0)))))))
    ;[1 1 1] Spawn an instance of the corridor builder at the correct vector and rotation
    (Game|SpawnActorfromClass "BP_CorridorBuilder_C" (Math|Transform|MakeTransform (Variables|Setup-Connection|GetSpawnVector) (Variables|Setup-Connection|GetSpawnRotation)) "Undefined" 0 0)))

(fn ConstructionScript
  (bind _spline (Variables|Default|GetSpline))
  (bind _spline_2 (Variables|Default|GetSpline))
  (bind _spline_3 (Variables|Default|GetSpline))
  (bind _returnvalue (Spline|GetNumberOfSplinePoints _spline_2))
  (bind _returnvalue_2 (Spline|GetNumberOfSplinePoints _spline_3))
  (for _index (range 0 (- (Spline|GetNumberOfSplinePoints (Variables|Default|GetSpline)) 2))
    (Variables|Setup-General|SetCurrentIndex _index)
    ;[1 1 1] For each spline point, add a mesh component and attach it
    (bind _returnvalue_3 (AddComponent|AddSplineMeshComponent false))
    (Variables|Default|SetSplineMeshComponent _returnvalue_3)
    (Transformation|AttachComponentToComponent _returnvalue_3 (Variables|Default|GetDefaultSceneRoot) "None" "KeepRelative" "KeepRelative" "KeepRelative" true)
    ;[1 1 1] Set the mesh component start and end positions
    (SplineMesh|SetStartandEnd _returnvalue_3 (.Location (Spline|GetLocationandTangentatSplinePoint _spline (Variables|Setup-General|GetCurrentIndex) "Local")) (.Tangent (Spline|GetLocationandTangentatSplinePoint _spline (Variables|Setup-General|GetCurrentIndex) "Local")) (.Location (Spline|GetLocationandTangentatSplinePoint _spline (+ (Variables|Setup-General|GetCurrentIndex) 1) "Local")) (.Tangent (Spline|GetLocationandTangentatSplinePoint _spline (+ (Variables|Setup-General|GetCurrentIndex) 1) "Local")) true :!class /Script/Engine.SplineMeshComponent)
    ;[1 1 1] Set the base and highlight materials
    (Rendering|Material|SetMaterial (Variables|Default|GetSplineMeshComponent) 0 (Variables|Setup-General|GetBaseMaterial))
    (Rendering|Material|SetMaterial (Variables|Default|GetSplineMeshComponent) 1 (Variables|Setup-General|GetHighlightMaterial))
    ;[1 1 1] Add spline index - this makes it easy to determine the spline point
    (bind _returnvalue_4 (AddComponent|AddTextRenderComponent false))
    (Transformation|SetRelativeLocation _returnvalue_4 (Spline|GetLocationatSplinePoint (Variables|Default|GetSpline) (Variables|Setup-General|GetCurrentIndex) "Local") false true)
    (Transformation|SetRelativeRotation _returnvalue_4 "0,180.000000, 0" false false)
    (Development|SetHiddeninGame _returnvalue_4 true false)
    (Rendering|Components|TextRender|SetText _returnvalue_4 (Utilities|Text|ToText(Integer) (Variables|Setup-General|GetCurrentIndex)))
    (Rendering|Components|TextRender|SetWorldSize _returnvalue_4 5e+02)
    (Rendering|Components|TextRender|SetTextRenderColor _returnvalue_4 (Math|Color|MakeColor 0 0 255 1)))
  (Utilities|FlowControl|Sequence
    (:then_0
      ;[1 1 1] Add last spline point
      (bind _returnvalue_5 (AddComponent|AddTextRenderComponent false))
      (Transformation|SetRelativeLocation _returnvalue_5 (Spline|GetLocationatSplinePoint _spline_3 _returnvalue_2 "Local") false true)
      (Transformation|SetRelativeRotation _returnvalue_5 "0,180.000000, 0" false false)
      (Development|SetHiddeninGame _spline_3 true false)
      (Rendering|Components|TextRender|SetText _returnvalue_5 (Utilities|Text|ToText(Integer) (- _returnvalue_2 1)))
      (Rendering|Components|TextRender|SetWorldSize _returnvalue_5 5e+02)
      (Rendering|Components|TextRender|SetTextRenderColor _returnvalue_5 (Math|Color|MakeColor 0 0 255 1)))
    (:then_1
      ;[1 1 1] Add End Mesh
      ;;[1 1 1] Add end mesh?
      (if (Variables|Setup-General|GetAddEndMesh?)
        ;;[1 1 1] Determine joint type to spawn
        (switch Utilities|FlowControl|Switch|SwitchonEnum_CorridorJointType (Variables|Setup-General|GetJointType)
          (:NewEnumerator0
            (Variables|Joints|SetSelectedMesh (Variables|Joints|GetMesh_Joint_Left)))
          (:NewEnumerator1
            (Variables|Joints|SetSelectedMesh (Variables|Joints|GetMesh_Joint_Right)))
          (:NewEnumerator2
            (Variables|Joints|SetSelectedMesh (Variables|Joints|GetMesh_Joint_Closed)))
          (:NewEnumerator3
            (Variables|Joints|SetSelectedMesh (Variables|Joints|GetMesh_Joint_T)))
          (:NewEnumerator4
            (Variables|Joints|SetSelectedMesh (Variables|Joints|GetMesh_Joint_Y))))
        ;;[1 1 1] Set the static mesh to the approriate joint
        (Components|StaticMesh|SetStaticMesh (Variables|Default|GetEndStaticMesh) (Variables|Joints|GetSelectedMesh))
        ;;[1 1 1] Set the location and rotation of the static mesh
        (Transformation|SetWorldLocationAndRotation (Variables|Default|GetEndStaticMesh) (Spline|GetLocationatSplinePoint _spline_2 _returnvalue "World") (Spline|GetRotationatSplinePoint _spline_2 _returnvalue "World") false true)))))