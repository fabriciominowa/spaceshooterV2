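; Procedural debris field actor that scatters randomly transformed instances of one mesh within a bounds box.
; The construction script fills an InstancedStaticMesh, seeds a per-instance health map and optionally culls instances inside a cull volume.
; Optional rotation spins the whole actor or rolls instances on a looping timer.
; Point damage depletes instance health, then zero-scales dead instances to preserve map indices and spawns BP_DestructibleObstacle in their place, optionally destroyed later.
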(event EventBeginPlay
  (Utilities|FlowControl|Sequence
    (:then_0
      ;[1 1 1] Rotate the instances?
      (if (Variables|Rotation|GetRotateInstances?)
        (CallFunction|EventRotateDebris)))
    (:then_1
      ;[1 1 1] Set rotation rate for this actor (entire field)
      (Variables|/Script/Engine.RotatingMovementComponent|SetRotationRate (Variables|Default|GetRotatingMovement) (Variables|Rotation|GetActorRotationRate)))))

(fn ConstructionScript
  (bind _bounds (Variables|Default|GetBounds))
  (bind _cullvolume (Variables|Default|GetCullVolume))
  (bind _bounds_2 (Variables|Default|GetBounds))
  ;[1 1 1] Activate RotatingMovement?
  (Components|Activation|SetAutoActivate (Variables|Default|GetRotatingMovement) (Variables|Rotation|GetUseActorRotation?))
  ;[1 1 1] Set scale for text renderer and billboard
  (Transformation|SetWorldScale3D (Variables|Default|GetTextRender) "1.000000,1.000000,1.000000")
  (Transformation|SetWorldScale3D (Variables|Default|GetBillboard) "5.000000,5.000000,5.000000")
  ;[1 1 1] Set Bound Scale
  (Transformation|SetWorldScale3D (Variables|Default|GetBounds) (Variables|Setup|GetBoundsScale))
  ;[1 1 1] Set Box Extent to size of the bounds collision box
  (Variables|/Script/Engine.SceneComponent|SetbAbsoluteScale _bounds true)
  (Components|Box|SetBoxExtent _bounds (.BoxExtent (Collision|GetComponentBounds _bounds)) true)
  ;[1 1 1] Set static mesh and material
  (Components|StaticMesh|SetStaticMesh (Variables|Default|GetInstancedStaticMesh) (Variables|Setup|GetStaticMesh))
  (Rendering|Material|SetMaterial (Variables|Default|GetInstancedStaticMesh) 0 (Variables|Setup|GetMeshMaterial))
  ;[1 1 1] Set Cull Volume scale and box extent
  (Transformation|SetWorldScale3D (Variables|Default|GetCullVolume) (Variables|Setup|GetCullVolumeScale))
  (Variables|/Script/Engine.SceneComponent|SetbAbsoluteScale _cullvolume true)
  (Components|Box|SetBoxExtent _cullvolume (.BoxExtent (Collision|GetComponentBounds _cullvolume)) true)
  (for _index (range 1 (Variables|Setup|GetNumberOfInstances))
    ;[1 1 1] Spawn new instance with random location, rotation, and scale
    (bind _returnvalue (Class|InstancedStaticMeshComponent|AddInstanceWorldSpace (Variables|Default|GetInstancedStaticMesh) (Math|Transform|MakeTransform (Math|Random|RandomPointinBoundingBox (Transformation|GetWorldLocation _bounds_2) (Components|Box|GetScaledBoxExtent _bounds_2)) (Math|Rotator|MakeRotator (Math|Random|RandomFloatinRange (Variables|Random|GetMinRandomRoll) (Variables|Random|GetMaxRandomRoll)) (Math|Random|RandomFloatinRange (Variables|Random|GetMinRandomPitch) (Variables|Random|GetMaxRandomPitch)) (Math|Random|RandomFloatinRange (Variables|Random|GetMinRandomYaw) (Variables|Random|GetMaxRandomYaw))) (Math|Vector|MakeVector (Math|Random|RandomFloatinRange (Variables|Random|GetMinRandomScale) (Variables|Random|GetMaxRandomScale)) (Math|Random|RandomFloatinRange (Variables|Random|GetMinRandomScale) (Variables|Random|GetMaxRandomScale)) (Math|Random|RandomFloatinRange (Variables|Random|GetMinRandomScale) (Variables|Random|GetMaxRandomScale))))))
    ;[1 1 1] Populate Map with instanceIndex and health
    (Utilities|Map|Add (Variables|Damage|GetInstanceHealthMap) _returnvalue (Variables|Damage|GetInstanceHealth)))
  (if (Variables|Setup|GetUseCullVolume?)
    ;[1 1 1] Cull instances inside the Cull Volume
    (CallFunction|FnGetInstancesInsideCullVolume)))

(fn FnIsInsideCullVolume
  (params (RandomVector :type Vector))
  (bind _cullvolume (Variables|Default|GetCullVolume))
  (bind _returnvalue (Transformation|GetWorldLocation _cullvolume))
  (bind _returnvalue_2 (Components|Box|GetScaledBoxExtent _cullvolume))
  (LocalVariables|SetTargetVector RandomVector)
  ;[1 1 1] Calculate Min and Max vectors
  (LocalVariables|SetxMin (- (.x _returnvalue) (.x _returnvalue_2)))
  (LocalVariables|SetxMax (+ (.x _returnvalue) (.x _returnvalue_2)))
  (LocalVariables|SetyMin (- (.y _returnvalue) (.y _returnvalue_2)))
  (LocalVariables|SetyMax (+ (.y _returnvalue) (.y _returnvalue_2)))
  (LocalVariables|SetzMin (- (.z _returnvalue) (.z _returnvalue_2)))
  (LocalVariables|SetzMax (+ (.z _returnvalue) (.z _returnvalue_2)))
  (if (Math|Boolean|ANDBoolean (<= (.x (LocalVariables|GetTargetVector)) (LocalVariables|GetxMax)) (>= (.x (LocalVariables|GetTargetVector)) (LocalVariables|GetxMin)) (<= (.y (LocalVariables|GetTargetVector)) (LocalVariables|GetyMax)) (>= (.y (LocalVariables|GetTargetVector)) (LocalVariables|GetyMin)) (<= (.z (LocalVariables|GetTargetVector)) (LocalVariables|GetzMax)) (>= (.z (LocalVariables|GetTargetVector)) (LocalVariables|GetzMin)))
    (return true)
    (else
      (return false))))

(fn FnGetInstancesInsideCullVolume
  (bind _cullvolume (Variables|Default|GetCullVolume))
  (bind _cullvolume_2 (Variables|Default|GetCullVolume))
  (bind _cullvolume_3 (Variables|Default|GetCullVolume))
  (bind _returnvalue (Transformation|GetWorldLocation _cullvolume_3))
  (bind _returnvalue_2 (Components|Box|GetScaledBoxExtent _cullvolume_3))
  (bind _returnvalue_3 (Transformation|GetWorldLocation _cullvolume))
  (bind _returnvalue_4 (Components|Box|GetScaledBoxExtent _cullvolume))
  (bind _returnvalue_5 (Transformation|GetWorldLocation _cullvolume_2))
  (bind _returnvalue_6 (Components|Box|GetScaledBoxExtent _cullvolume_2))
  ;[1 1 1] Calculate Min and Max vectors
  (LocalVariables|SetxMin (- (.x _returnvalue_3) (.x _returnvalue_4)))
  (LocalVariables|SetxMax (+ (.x _returnvalue_3) (.x _returnvalue_4)))
  (LocalVariables|SetyMin (- (.y _returnvalue_5) (.y _returnvalue_6)))
  (LocalVariables|SetyMax (+ (.y _returnvalue_5) (.y _returnvalue_6)))
  (LocalVariables|SetzMin (- (.z _returnvalue) (.z _returnvalue_2)))
  (LocalVariables|SetzMax (+ (.z _returnvalue) (.z _returnvalue_2)))
  (bind _output_get (LocalVariables|SetInstancesToRemove (Class|InstancedStaticMeshComponent|GetInstancesOverlappingBox (Variables|Default|GetInstancedStaticMesh) (Math|Box|MakeBox (Math|Vector|MakeVector (LocalVariables|GetxMin) (LocalVariables|GetyMin) (LocalVariables|GetzMin)) (Math|Vector|MakeVector (LocalVariables|GetxMax) (LocalVariables|GetyMax) (LocalVariables|GetzMax))) true)))
  (for _array_element _output_get
    ;[1 1 1] Remove all overlapping instances starting at the highest index (to prevent order from changing)
    (LocalVariables|SetIndexOfMaxValue (.IndexOfMaxValue (Math|Integer|MaxOfIntArray (LocalVariables|GetInstancesToRemove))))
    (bind _output_get_2 (LocalVariables|SetMaxValue (.MaxValue (Math|Integer|MaxOfIntArray (LocalVariables|GetInstancesToRemove)))))
    (Class|InstancedStaticMeshComponent|RemoveInstance (Variables|Default|GetInstancedStaticMesh) _output_get_2)
    (Utilities|Array|SetArrayElem (LocalVariables|GetInstancesToRemove) (LocalVariables|GetIndexOfMaxValue) -1)
    ;[1 1 1] Populate Map with instanceIndex and health
    (Utilities|Map|Remove (Variables|Damage|GetInstanceHealthMap) (LocalVariables|GetMaxValue)))
  ;[1 1 1] Clear array
  (Utilities|Array|Clear (LocalVariables|GetInstancesToRemove)))

(event Custom|EventRotateDebris
  (bind _instancedstaticmesh (Variables|Default|GetInstancedStaticMesh))
  (bind _outinstancetransform (Components|InstancedStaticMesh|GetInstanceTransform _instancedstaticmesh 0 true))
  (Utilities|Time|SetTimerbyEvent (delegate Custom|EventRotateDebris) (Variables|Rotation|GetRotationTimer) true)
  ;[1 1 1] Go through all instances of the ISM component
  (for _index (range 0 (Components|InstancedStaticMesh|GetInstanceCount (Variables|Default|GetInstancedStaticMesh)))
    ;[1 1 1] Rotate all instances
    (Components|InstancedStaticMesh|UpdateInstanceTransform (Variables|Default|GetInstancedStaticMesh) _index (Math|Transform|MakeTransform (.location (.OutInstanceTransform (Components|InstancedStaticMesh|GetInstanceTransform (Variables|Default|GetInstancedStaticMesh) _index true))) (Math|Rotator|MakeRotator (+ (.roll (.rotation (.OutInstanceTransform (Components|InstancedStaticMesh|GetInstanceTransform (Variables|Default|GetInstancedStaticMesh) _index true)))) 1.0) (.pitch (.rotation (.OutInstanceTransform (Components|InstancedStaticMesh|GetInstanceTransform (Variables|Default|GetInstancedStaticMesh) _index true)))) (.yaw (.rotation (.OutInstanceTransform (Components|InstancedStaticMesh|GetInstanceTransform (Variables|Default|GetInstancedStaticMesh) _index true))))) (.scale (.OutInstanceTransform (Components|InstancedStaticMesh|GetInstanceTransform (Variables|Default|GetInstancedStaticMesh) _index true)))) true true true))
  ;[1 1 1] Rotate all instances
  (Components|InstancedStaticMesh|UpdateInstanceTransform (Variables|Default|GetInstancedStaticMesh) (Components|InstancedStaticMesh|GetInstanceCount (Variables|Default|GetInstancedStaticMesh)) (Math|Transform|MakeTransform (.location _outinstancetransform) (.rotation _outinstancetransform) (.scale _outinstancetransform)) true true true))

(event OnComponentHit(InstancedStaticMesh)
  (params (HitComponent :type Primitive%20Component%20Object%20Reference) (OtherActor :type Actor%20Object%20Reference) (OtherComp :type Primitive%20Component%20Object%20Reference) (NormalImpulse :type Vector :default "0, 0, 0") (Hit :type Hit%20Result%20Structure%20%28by%20ref%29))
  (bind (_bblockinghit _binitialoverlap _time _distance _location _impactpoint _normal _impactnormal _physmat _hitactor _hitcomponent _hitbonename _hititem) (Collision|BreakHitResult Hit))
  ;[1 1 1] Do the instances take damage?
  (if (Variables|Damage|GetTakeDamage?)
    ;[1 1 1] Record instance hit, as well as hit location and normal
    (bind _output_get (Variables|Damage|SetInstanceHit _hititem))
    (Variables|Damage|SetImpactLocation _impactpoint)
    (Variables|Damage|SetImpactNormal _impactnormal)))

(event Game|Damage|EventPointDamage
  (params (Damage :type Float%20%28single-precision%29) (DamageType :type Damage%20Type%20Object%20Reference) (HitLocation :type Vector :default "0, 0, 0") (HitNormal :type Vector :default "0, 0, 0") (HitComponent :type Primitive%20Component%20Object%20Reference) (BoneName :type Name :default "None") (ShotFromDirection :type Vector :default "0, 0, 0") (InstigatedBy :type Controller%20Object%20Reference) (DamageCauser :type Actor%20Object%20Reference) (HitInfo :type Hit%20Result%20Structure%20%28by%20ref%29))
  (bind (_bblockinghit _binitialoverlap _time _distance _location _impactpoint _normal _impactnormal _physmat _hitactor _hitcomponent _hitbonename _hititem) (Collision|BreakHitResult HitInfo))
  (Utilities|FlowControl|Delay 0.1)
  ;[1 1 1] Set damage parameters
  (Variables|Damage|SetDamageTaken Damage)
  (Variables|Damage|SetInstanceHit _hititem)
  (Variables|Damage|SetImpactLocation _impactpoint)
  (Variables|Damage|SetImpactNormal _impactnormal)
  ;[1 1 1] Reduce Health of instance by damage taken
  (Utilities|Map|Add (Variables|Damage|GetInstanceHealthMap) (Variables|Damage|GetInstanceHit) (- (.Value (Utilities|Map|Find (Variables|Damage|GetInstanceHealthMap) (Variables|Damage|GetInstanceHit))) (Variables|Damage|GetDamageTaken)))
  ;[1 1 1] If Health is 0 or less
  (if (<= (.Value (Utilities|Map|Find (Variables|Damage|GetInstanceHealthMap) (Variables|Damage|GetInstanceHit))) 0.0)
    ;[1 1 1] Save ISM instance transform
    (Variables|Damage|SetNewDMTransform (.OutInstanceTransform (Components|InstancedStaticMesh|GetInstanceTransform (Variables|Default|GetInstancedStaticMesh) (Variables|Damage|GetInstanceHit) true)))
    ;[1 1 1] Scale ISM instance to 0 to "remove it" - Do this instead of removing it to preserve index values synced with Map
    (Components|InstancedStaticMesh|UpdateInstanceTransform (Variables|Default|GetInstancedStaticMesh) (Variables|Damage|GetInstanceHit) (Math|Transform|MakeTransform "0, 0, 0" "0, 0, 0" "0.000000,0.000000,0.000000") true true false)
    ;[1 1 1] Spawn destructible Obstacle and set the destructible mesh to DestructibleMesh
    (bind _returnvalue (Game|SpawnActorfromClass "/Game/ASST/Blueprints/Actors/Obstacles/BP_DestructibleObstacle.BP_DestructibleObstacle_C" (Variables|Damage|GetNewDMTransform) "AlwaysSpawn" 0 0))
    (Variables|Damage|SetSpawnedDM _returnvalue)
    ;[1 1 1] Set DM mesh to DestructibleMesh
    (Variables|/Game/ASST/Blueprints/Actors/Obstacles/BP_DestructibleObstacle.BP_DestructibleObstacle_C|SetDestructibleMesh (Variables|Damage|GetSpawnedDM) (Variables|Setup|GetDestructibleMesh))
    ;[1 1 1] Set DM mesh materials
    (Rendering|Material|SetMaterial (Variables|/Game/ASST/Blueprints/Actors/Obstacles/BP_DestructibleObstacleParent.BP_DestructibleObstacleParent_C|GetDestructible (Variables|Damage|GetSpawnedDM)) 0 (Variables|Setup|GetMeshMaterial))
    (Rendering|Material|SetMaterial (Variables|/Game/ASST/Blueprints/Actors/Obstacles/BP_DestructibleObstacleParent.BP_DestructibleObstacleParent_C|GetDestructible (Variables|Damage|GetSpawnedDM)) 1 (Variables|Setup|GetMeshMaterial))
    ;[1 1 1] Does the DM debris have collision?
    (if (not (Variables|Damage|GetDebrisHasCollision?))
      (Utilities|FlowControl|Delay 0.5)
      (Collision|SetCollisionEnabled (Variables|/Game/ASST/Blueprints/Actors/Obstacles/BP_DestructibleObstacleParent.BP_DestructibleObstacleParent_C|GetDestructible (Variables|Damage|GetSpawnedDM)) "NoCollision"))
    ;[1 1 1] Destroy Actor
    (if (Variables|Damage|GetDestroyDM?)
      ;;[1 1 1] Check if Spawned DM has a DelayedDeath component
      (if (Utilities|IsValid (Actor|GetComponentbyClass (Variables|Damage|GetSpawnedDM) "/Game/ASST/Blueprints/Actors/Components/BP_CompDelayedDeath.BP_CompDelayedDeath_C"))
        ;;[1 1 1] Set delayed death amount
        (Default|EventDelayDeath (Actor|GetComponentbyClass (Variables|Damage|GetSpawnedDM) "/Game/ASST/Blueprints/Actors/Components/BP_CompDelayedDeath.BP_CompDelayedDeath_C") (Variables|Damage|GetDestroyDelay))
        (else
          ;;[1 1 1] No component found - simply use a delay and destroy the actor
          (Utilities|FlowControl|Delay (Variables|Damage|GetDestroyDelay))
          (Actor|DestroyActor (Variables|Damage|GetSpawnedDM)))))))