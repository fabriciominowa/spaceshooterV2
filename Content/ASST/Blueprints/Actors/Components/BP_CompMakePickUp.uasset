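; Actor component that turns its owner into a pickup, reacting when any actor begins overlapping it.
; On BeginPlay it binds to the owner's begin-overlap event; each overlap plays the pickup sound and optionally destroys the owner.
; When radar removal is enabled, it first waits briefly, then removes the owner by category (flying enemy, ground enemy, boss or pickup) through the radar widget held by BP_FlyingGameInstance.
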(event Custom|EventOverlap
  (params (OverlappedActor :type Actor%20Object%20Reference) (OtherActor :type Actor%20Object%20Reference))
  ;[1 1 1] Bind On Overlap Event
  (if (Variables|Setup|GetRemoveFromRadar?)
    (CallFunction|EventRemovefromRadar)
    (else
      (Audio|PlaySound2D (Variables|Setup|GetPickUpSound))
      ;[1 1 1] Destroy Actor
      (if (Variables|Setup|GetDestroyActor?)
        (Actor|DestroyActor (Components|GetOwner))))))

(event EventBeginPlay
  ;[0 0.1011 1] Make sure you enable 'Generate Overlap Events and make actor 'Overlap All Dynamic'
  ;[1 1 1] Get Primitive Component
  (Variables|Default|SetPrimitiveComponent (Utilities|Array|Get(acopy) (Actor|GetComponentsByClass (Components|GetOwner) "/Script/Engine.PrimitiveComponent")))
  ;[1 1 1] Bind On Overlap Event
  (EventDispatchers|AssignOnActorBeginOverlap (Components|GetOwner (Variables|Default|GetPrimitiveComponent)) (delegate Custom|EventOverlap)))

(event Custom|EventRemoveFromRadar
  (switch Utilities|FlowControl|Switch|SwitchonEnum_RadarCategories (Variables|Setup|GetRadarCategory)
    (:NewEnumerator0
      ;[1 1 1] Remove Flying Enemy from Radar
      (Utilities|FlowControl|Delay 0.1)
      (bind _asbp_flying_game_instance (Utilities|Casting|CastToBP_FlyingGameInstance (Game|GetGameInstance)))
      (Default|FnRemoveFlyingEnemy (Variables|/Game/ASST/Blueprints/BP_FlyingGameInstance.BP_FlyingGameInstance_C|GetWBPRadarRef _asbp_flying_game_instance) (Components|GetOwner)))
    (:NewEnumerator1
      ;[1 1 1] Remove Ground Enemy from Radar
      (Utilities|FlowControl|Delay 0.1)
      (bind _asbp_flying_game_instance_2 (Utilities|Casting|CastToBP_FlyingGameInstance (Game|GetGameInstance)))
      (Default|FnRemoveGroundEnemy (Variables|/Game/ASST/Blueprints/BP_FlyingGameInstance.BP_FlyingGameInstance_C|GetWBPRadarRef _asbp_flying_game_instance_2) (Components|GetOwner)))
    (:NewEnumerator2
      ;[1 1 1] Remove Boss from Radar
      (Utilities|FlowControl|Delay 0.1)
      (bind _asbp_flying_game_instance_3 (Utilities|Casting|CastToBP_FlyingGameInstance (Game|GetGameInstance)))
      (Default|FnRemoveBoss (Variables|/Game/ASST/Blueprints/BP_FlyingGameInstance.BP_FlyingGameInstance_C|GetWBPRadarRef _asbp_flying_game_instance_3) (Components|GetOwner)))
    (:NewEnumerator3
      ;[1 1 1] Add PickUp to Radar
      (Utilities|FlowControl|Delay 0.1)
      (bind _asbp_flying_game_instance_4 (Utilities|Casting|CastToBP_FlyingGameInstance (Game|GetGameInstance)))
      (Default|FnRemovePickUp (Variables|/Game/ASST/Blueprints/BP_FlyingGameInstance.BP_FlyingGameInstance_C|GetWBPRadarRef _asbp_flying_game_instance_4) (Components|GetOwner))))
  (Audio|PlaySound2D (Variables|Setup|GetPickUpSound))
  ;[1 1 1] Destroy Actor
  (if (Variables|Setup|GetDestroyActor?)
    (Actor|DestroyActor (Components|GetOwner))))