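; Actor component that makes its owner hover in place, bobbing up and down around its starting relative Z height.
; BeginPlay caches the first primitive component and its Z, then starts the hover if it is Movable, otherwise printing an error.
; A looping timer re-runs the hover event, flipping direction at the ZOffset limits.
; Each step applies a swept local offset sized by FInterpTo and world delta time.
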(event EventBeginPlay
  ;[1 1 1] Grab primitive component
  (Variables|Default|SetPrimitiveComponent (Utilities|Array|Get(acopy) (Actor|GetComponentsByClass (Components|GetOwner) "/Script/Engine.PrimitiveComponent")))
  ;[1 1 1] Save starting Z offset
  (Variables|Default|SetStartingZOffset (.z (Variables|/Script/Engine.SceneComponent|GetRelativeLocation (Variables|Default|GetPrimitiveComponent))))
  ;[1 1 1] Check to see if actor is Movable
  (if (Utilities|Enum|Equal(Enum) (Variables|/Script/Engine.SceneComponent|GetMobility (Variables|Default|GetPrimitiveComponent)) "Movable")
    (CallFunction|EventHoverinPlace)
    (else
      ;[1 1 1] Actor NOT movable - Display ERROR
      (Development|PrintString (Utilities|String|Append (Variables|Default|GetErrorText1) (Utilities|GetDisplayName (Components|GetOwner (Variables|Default|GetPrimitiveComponent))) (Variables|Default|GetErrorText2)) true true "(R=0.000000,G=0.660000,B=1.000000,A=1.000000)" 1e+01))))

(event Custom|EventHoverInPlace
  (Utilities|Time|SetTimerbyEvent (delegate Custom|EventHoverInPlace) 0.01 true)
  (if (Variables|Default|GetGoingUp?)
    ;[1 1 1] Check upper limits
    (if (>= (.z (Variables|/Script/Engine.SceneComponent|GetRelativeLocation (Variables|Default|GetPrimitiveComponent))) (+ (Variables|Default|GetStartingZOffset) (Variables|Setup|GetZOffset)))
      (Variables|Default|SetGoingUp? false)
      (else
        (CallFunction|EventGoUp)))
    (else
      ;[1 1 1] Check lower limits
      (if (>= (- (.z (Variables|/Script/Engine.SceneComponent|GetRelativeLocation (Variables|Default|GetPrimitiveComponent))) (Variables|Default|GetStartingZOffset)) (* (Variables|Setup|GetZOffset) -1.0))
        (CallFunction|EventGoDown)
        (else
          (Variables|Default|SetGoingUp? true))))))

(event Custom|EventGoUp
  ;[1 1 1] Add Local Offset to Z
  (Transformation|AddLocalOffset (Variables|Default|GetPrimitiveComponent) (Math|Vector|MakeVector 0.0 0.0 (Math|Interpolation|FInterpTo 0.0 (* (Variables|Setup|GetZOffset) 1.0) (Utilities|Time|GetWorldDeltaSeconds) 1.0)) true false))

(event Custom|EventGoDown
  ;[1 1 1] Add Local Offset to Z
  (Transformation|AddLocalOffset (Variables|Default|GetPrimitiveComponent) (Math|Vector|MakeVector 0.0 0.0 (Math|Interpolation|FInterpTo 0.0 (* (Variables|Setup|GetZOffset) -1.0) (Utilities|Time|GetWorldDeltaSeconds) 1.0)) true false))