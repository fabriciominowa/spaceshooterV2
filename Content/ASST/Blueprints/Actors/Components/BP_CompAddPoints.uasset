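; Actor component that awards points to the player when its owning actor is hit.
; On BeginPlay it reaches the owner through its first primitive component and binds to that actor's hit event.
; Each hit, whatever the other actor, sends PointsToAdd to player pawn 0 through the BPIAddPoints interface, with an AddPointsOnce flag and DoOnce intended to limit it to one award.
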(event Custom|EventHit
  (params (SelfActor :type Actor%20Object%20Reference) (OtherActor :type Actor%20Object%20Reference) (NormalImpulse :type Vector) (Hit :type Hit%20Result%20Structure%20%28by%20ref%29))
  ;[1 1 1] Bind OnActorHit Event and call fnAddPoints from BPIAddPoints
  (if (Variables|Setup|GetAddPointsOnce?)
    (Utilities|FlowControl|DoOnce false
      (:Completed
        _)))
  (Class|BPBPIPlayerConn|FnBPIAddPoints(Message) (Game|Player|GetPlayerPawn 0) (Variables|Setup|GetPointsToAdd)))

(event EventBeginPlay
  ;[1 1 1] Get primitive component from owner
  (bind _output_get (Variables|Default|SetPrimitiveComponent (Utilities|Array|Get(acopy) (Actor|GetComponentsByClass (Components|GetOwner) "/Script/Engine.PrimitiveComponent"))))
  ;[1 1 1] Bind OnActorHit Event and call fnAddPoints from BPIAddPoints
  (Collision|BindEventtoOnActorHit (Components|GetOwner _output_get) (delegate Custom|EventHit)))