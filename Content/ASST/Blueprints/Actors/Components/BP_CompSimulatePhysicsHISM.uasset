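; Actor component that makes instances of the owner's Hierarchical Instanced Static Mesh breakable into physics-simulating actors.
; It maps instance indices to hit-count health, and each owner hit decrements the struck instance after a short delay.
; At zero, it swaps the instance for a spawned DMClass actor pushed along the impact normal, printing an error if not Movable.
; Optionally, that actor is destroyed later, via BP_CompDelayedDeath when present.
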(event Custom|EventHit
  (params (SelfActor :type Actor%20Object%20Reference) (OtherActor :type Actor%20Object%20Reference) (NormalImpulse :type Vector) (Hit :type Hit%20Result%20Structure%20%28by%20ref%29))
  (bind (_bblockinghit _binitialoverlap _time _location _impactpoint _normal _impactnormal _physmat _hitactor _hitcomponent _hitbonename _hititem) (Collision|BreakHitResult Hit))
  ;[1 1 1] Bind OnActorHit event
  ;[1 1 1] Save hit instance and hit location and normal
  (Variables|Default|SetInstanceHit _hititem)
  (Variables|Default|SetHitLocation _impactpoint)
  (Variables|Default|SetImpactNormal _impactnormal)
  ;[1 1 1] Apply damage to the instance
  (CallFunction|EventApplyDamage))

(event EventBeginPlay
  ;[1 1 1] Populate health map
  (CallFunction|EventPopulateHealthMap)
  ;[1 1 1] Bind OnActorHit event
  (Collision|BindEventtoOnActorHit (Components|GetOwner) (delegate Custom|EventHit)))

(event Custom|EventPopulateHealthMap
  ;[1 1 1] Go through all the instances in the HISM component
  (for _index (range 0 (- (Components|InstancedStaticMesh|GetInstanceCount (Actor|GetComponentbyClass (Components|GetOwner) "/Script/Engine.HierarchicalInstancedStaticMeshComponent")) 1))
    ;[1 1 1] Create a new map entry for each instance with the InstanceHealth
    (Utilities|Map|Add (Variables|Default|GetInstanceHealthMap) _index (Variables|Setup|GetInstanceHealth))))

(event Custom|EventApplyDamage
  (bind _destructiondelay (Variables|Setup|GetDestructionDelay))
  (Utilities|FlowControl|Delay 0.2)
  ;[1 1 1] Reduce Health by 1 hit
  (Utilities|Map|Add (Variables|Default|GetInstanceHealthMap) (Variables|Default|GetInstanceHit) (- (.Value (Utilities|Map|Find (Variables|Default|GetInstanceHealthMap) (Variables|Default|GetInstanceHit))) 1))
  ;[1 1 1] Check if the instance's health reached 0
  (if (<= (.Value (Utilities|Map|Find (Variables|Default|GetInstanceHealthMap) (Variables|Default|GetInstanceHit))) 0)
    ;[1 1 1] Save instance transform before removing it
    (Variables|Default|SetNewDMTransform (.OutInstanceTransform (Components|InstancedStaticMesh|GetInstanceTransform (Actor|GetComponentbyClass (Components|GetOwner) "/Script/Engine.HierarchicalInstancedStaticMeshComponent") (Variables|Default|GetInstanceHit) true)))
    ;[1 1 1] Remove instance
    (Class|InstancedStaticMeshComponent|RemoveInstance (Actor|GetComponentbyClass (Components|GetOwner) "/Script/Engine.HierarchicalInstancedStaticMeshComponent") (Variables|Default|GetInstanceHit))
    ;[1 1 1] Spawn destructible actor with the mesh specified
    (bind _returnvalue (Game|SpawnActorfromClass (Variables|Setup|GetDM_Class) (Variables|Default|GetNewDMTransform) "AlwaysSpawn" 0 0))
    (Variables|Default|SetRef _returnvalue)
    ;[1 1 1] Remove map element
    (Utilities|Map|Remove (Variables|Default|GetInstanceHealthMap) (Variables|Default|GetInstanceHit))
    ;[1 1 1] Check if mesh is movable
    (if (Utilities|Enum|Equal(Enum) (Variables|/Script/Engine.SceneComponent|GetMobility (Actor|GetComponentbyClass (Variables|Default|GetRef) "/Script/Engine.PrimitiveComponent")) "Movable")
      ;[1 1 1] Simulate physics and apply damage to destructible mesh
      (Physics|SetSimulatePhysics (Actor|GetComponentbyClass (Variables|Default|GetRef) "/Script/Engine.PrimitiveComponent") true)
      (Physics|AddImpulseatLocation (Actor|GetComponentbyClass (Variables|Default|GetRef) "/Script/Engine.PrimitiveComponent") (* (Variables|Default|GetImpactNormal) (Variables|Setup|GetImpactImpulse)) (Variables|Default|GetHitLocation) "None")
      ;[1 1 1] Destroy Component, if appropriate
      (if (Variables|Setup|GetDestroyMesh?)
        (if (Utilities|IsValid (Actor|GetComponentbyClass (Variables|Default|GetRef) "/Game/ASST/Blueprints/Actors/Components/BP_CompDelayedDeath.BP_CompDelayedDeath_C"))
          (Default|EventDelayDeath (Actor|GetComponentbyClass (Variables|Default|GetRef) "/Game/ASST/Blueprints/Actors/Components/BP_CompDelayedDeath.BP_CompDelayedDeath_C") _destructiondelay)
          (else
            (Utilities|FlowControl|Delay _destructiondelay)
            (Actor|DestroyActor (Variables|Default|GetRef)))))
      (else
        ;[1 1 1] Display ERROR
        (Development|PrintString (Utilities|String|Append "Actor: " (Utilities|GetDisplayName (Variables|Default|GetRef)) " is NOT set to Movable!") true true "(R=0.000000,G=0.660000,B=1.000000,A=1.000000)" 1e+01)))))