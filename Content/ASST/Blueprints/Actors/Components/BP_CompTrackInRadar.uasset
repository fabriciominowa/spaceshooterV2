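; Actor component that registers its owning actor on the radar widget as a flying enemy, ground enemy, boss or pickup, according to its RadarCategory.
; On BeginPlay it waits briefly, then calls the matching add function on the radar widget reference held by BP_FlyingGameInstance.
; A separate removal event mirrors this with the matching remove functions, but nothing in this component calls it.
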(event EventBeginPlay
  (CallFunction|EventAddtoRadar))

(event Custom|EventAddToRadar
  (switch Utilities|FlowControl|Switch|SwitchonEnum_RadarCategories (Variables|Setup|GetRadarCategory)
    (:NewEnumerator0
      ;[1 1 1] Add Flying Enemy to Radar
      (Utilities|FlowControl|Delay 0.1)
      (bind _asbp_flying_game_instance (Utilities|Casting|CastToBP_FlyingGameInstance (Game|GetGameInstance)))
      (Default|FnAddFlyingEnemy (Variables|/Game/ASST/Blueprints/BP_FlyingGameInstance.BP_FlyingGameInstance_C|GetWBPRadarRef _asbp_flying_game_instance) (Components|GetOwner)))
    (:NewEnumerator1
      ;[1 1 1] Add Ground Enemy to Radar
      (Utilities|FlowControl|Delay 0.1)
      (bind _asbp_flying_game_instance_2 (Utilities|Casting|CastToBP_FlyingGameInstance (Game|GetGameInstance)))
      (Default|FnAddGroundEnemy (Variables|/Game/ASST/Blueprints/BP_FlyingGameInstance.BP_FlyingGameInstance_C|GetWBPRadarRef _asbp_flying_game_instance_2) (Components|GetOwner)))
    (:NewEnumerator2
      ;[1 1 1] Add Boss to Radar
      (Utilities|FlowControl|Delay 0.1)
      (bind _asbp_flying_game_instance_3 (Utilities|Casting|CastToBP_FlyingGameInstance (Game|GetGameInstance)))
      (Default|FnAddBoss (Variables|/Game/ASST/Blueprints/BP_FlyingGameInstance.BP_FlyingGameInstance_C|GetWBPRadarRef _asbp_flying_game_instance_3) (Components|GetOwner)))
    (:NewEnumerator3
      ;[1 1 1] Add PickUp to Radar
      (Utilities|FlowControl|Delay 0.1)
      (bind _asbp_flying_game_instance_4 (Utilities|Casting|CastToBP_FlyingGameInstance (Game|GetGameInstance)))
      (Default|FnAddPickUp (Variables|/Game/ASST/Blueprints/BP_FlyingGameInstance.BP_FlyingGameInstance_C|GetWBPRadarRef _asbp_flying_game_instance_4) (Components|GetOwner)))))

(event Custom|EventRemoveFromRadar
  (switch Utilities|FlowControl|Switch|SwitchonEnum_RadarCategories (Variables|Setup|GetRadarCategory)
    (:NewEnumerator0
      ;[1 1 1] Remove Flying Enemy from Radar
      (Utilities|FlowControl|Delay 0.1)
      (bind _asbp_flying_game_instance (Utilities|Casting|CastToBP_FlyingGameInstance (Game|GetGameInstance)))
      (Default|FnRemoveFlyingEnemy (Variables|/Game/ASST/Blueprints/BP_FlyingGameInstance.BP_FlyingGameInstance_C|GetWBPRadarRef _asbp_flying_game_instance) (Components|GetOwner)))
    (:NewEnumerator1
      ;[1 1 1] Remove Ground Enemy from Radar
      (Utilities|FlowControl|Delay 0.1)
      (bind _asbp_flying_game_instance_2 (Utilities|Casting|CastToBP_FlyingGameInstance (Game|GetGameInstance)))
      (Default|FnRemoveGroundEnemy (Variables|/Game/ASST/Blueprints/BP_FlyingGameInstance.BP_FlyingGameInstance_C|GetWBPRadarRef _asbp_flying_game_instance_2) (Components|GetOwner)))
    (:NewEnumerator2
      ;[1 1 1] Remove Boss from Radar
      (Utilities|FlowControl|Delay 0.1)
      (bind _asbp_flying_game_instance_3 (Utilities|Casting|CastToBP_FlyingGameInstance (Game|GetGameInstance)))
      (Default|FnRemoveBoss (Variables|/Game/ASST/Blueprints/BP_FlyingGameInstance.BP_FlyingGameInstance_C|GetWBPRadarRef _asbp_flying_game_instance_3) (Components|GetOwner)))
    (:NewEnumerator3
      ;[1 1 1] Add PickUp to Radar
      (Utilities|FlowControl|Delay 0.1)
      (bind _asbp_flying_game_instance_4 (Utilities|Casting|CastToBP_FlyingGameInstance (Game|GetGameInstance)))
      (Default|FnRemovePickUp (Variables|/Game/ASST/Blueprints/BP_FlyingGameInstance.BP_FlyingGameInstance_C|GetWBPRadarRef _asbp_flying_game_instance_4) (Components|GetOwner)))))