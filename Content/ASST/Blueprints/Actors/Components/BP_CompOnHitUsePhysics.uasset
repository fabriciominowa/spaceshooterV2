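; BP_CompOnHitUsePhysics is an actor component that turns its owner into a physics object when hit, optionally destroying it afterward.
; On BeginPlay it takes the owner's first primitive component and binds OnActorHit if that is Movable, otherwise printing an error.
; A hit enables physics and applies an impulse along the impact normal.
; If DestroyActor is set, it waits DestroyDelay, spawns an emitter and destroys the owner shortly after.
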(event Custom|OnActorHit_Event_0
  (params (SelfActor :type Actor%20Object%20Reference) (OtherActor :type Actor%20Object%20Reference) (NormalImpulse :type Vector) (Hit :type Hit%20Result%20Structure%20%28by%20ref%29))
  (bind (_bblockinghit _binitialoverlap _time _location _impactpoint _normal _impactnormal) (Collision|BreakHitResult Hit))
  (bind _primitivecomponent (Variables|Default|GetPrimitiveComponent))
  ;[1 1 1] Bind Hit Event and simulate physics and add impulse
  (Physics|SetSimulatePhysics _primitivecomponent true)
  (Physics|AddImpulseatLocation _primitivecomponent (* _impactnormal (Variables|Setup|GetImpulseOnDestroy)) _impactpoint "None")
  (if (Variables|Setup|GetDestroyActor?)
    ;[1 1 1] Delay by DestroyDelay, then spawn emitter and destroy actor
    (Utilities|FlowControl|Delay (Variables|Setup|GetDestroyDelay))
    (Effects|SpawnEmitterAttached (Variables|Setup|GetEmitter) (Variables|Default|GetPrimitiveComponent) "None" (Transformation|GetActorLocation (Components|GetOwner (Variables|Default|GetPrimitiveComponent))) "0, 0, 0" "KeepWorldPosition")
    (Utilities|FlowControl|Delay 0.5)
    (Actor|DestroyActor (Components|GetOwner (Variables|Default|GetPrimitiveComponent)))))

(event EventBeginPlay
  ;[1 1 1] Get Primitive Component
  (Variables|Default|SetPrimitiveComponent (Utilities|Array|Get(acopy) (Actor|GetComponentsByClass (Components|GetOwner) "/Script/Engine.PrimitiveComponent")))
  ;[1 1 1] Check to see if object is Movable
  (if (Utilities|Enum|Equal(Enum) (Variables|/Script/Engine.SceneComponent|GetMobility (Variables|Default|GetPrimitiveComponent)) "Movable")
    ;[1 1 1] Bind Hit Event and simulate physics and add impulse
    (Collision|AssignOnActorHit (Components|GetOwner (Variables|Default|GetPrimitiveComponent)) (delegate Custom|OnActorHit_Event_0))
    (else
      ;[1 1 1] Display ERROR
      (Development|PrintString (Utilities|String|Append (Variables|Default|GetErrorText1) (Utilities|GetDisplayName (Components|GetOwner (Variables|Default|GetPrimitiveComponent))) (Variables|Default|GetErrorText2)) true true "(R=0.000000,G=0.660000,B=1.000000,A=1.000000)" 1e+01))))