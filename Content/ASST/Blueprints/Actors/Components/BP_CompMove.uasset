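; BP_CompMove is an actor component that moves its owner's first primitive component by a local offset, optionally only while a player ship is nearby.
; On BeginPlay it caches the starting location and prints an error unless the primitive is Movable.
; A 0.01-second timer event drives the swept movement, gated by an optional sphere overlap for BP_PlayerShip, and can destroy the owner beyond a set distance from its start.
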(event EventBeginPlay
  ;[1 1 1] Get primitive component
  (Variables|Default|SetPrimitiveComponent (Utilities|Array|Get(acopy) (Actor|GetComponentsByClass (Components|GetOwner) "/Script/Engine.PrimitiveComponent")))
  ;[1 1 1] Save starting vector
  (Variables|Default|SetStartingVector (Variables|/Script/Engine.SceneComponent|GetRelativeLocation (Variables|Default|GetPrimitiveComponent)))
  ;[1 1 1] Check to see if object is Movable
  (if (Utilities|Enum|Equal(Enum) (Variables|/Script/Engine.SceneComponent|GetMobility (Variables|Default|GetPrimitiveComponent)) "Movable")
    (CallFunction|EventMove)
    (else
      ;[1 1 1] Display ERROR
      (Development|PrintString (Utilities|String|Append (Variables|Default|GetErrorText1) (Utilities|GetDisplayName (Components|GetOwner (Variables|Default|GetPrimitiveComponent))) (Variables|Default|GetErrorText2)) true true "(R=0.000000,G=0.660000,B=1.000000,A=1.000000)" 1e+01))))

(event Custom|EventMove
  (Utilities|Time|SetTimerbyEvent (delegate Custom|EventMove) 0.01 true)
  (Utilities|FlowControl|Sequence
    (:then_0
      (if (Variables|Setup|GetActivateOnProximity?)
        (bind _returnvalue (Collision|SphereOverlapActors (Transformation|GetWorldLocation (Variables|Default|GetPrimitiveComponent)) (Variables|Setup|GetProximityRadius) (Utilities|Array|MakeArray "ObjectTypeQuery3") "/Game/ASST/Blueprints/Characters/Player/BP_PlayerShip.BP_PlayerShip_C"))
        (if _returnvalue
          ;[1 1 1] Move actor by the offset vector
          (Transformation|AddLocalOffset (Variables|Default|GetPrimitiveComponent) (Variables|Setup|GetOffsetVector) true false :!label _label))
        (else
          (goto _label))))
    (:then_1
      (if (Variables|Setup|GetDestroyActor?)
        ;[1 1 1] Check the distance traveled by object. If bigger than DestroyOnDistance, destroy actor
        (if (>= (Math|Vector|VectorLength (- (Variables|/Script/Engine.SceneComponent|GetRelativeLocation (Variables|Default|GetPrimitiveComponent)) (Variables|Default|GetStartingVector))) (Variables|Setup|GetDestroyOnDistance))
          ;[1 1 1] Destroy actor
          (Actor|DestroyActor (Components|GetOwner (Variables|Default|GetPrimitiveComponent))))))))