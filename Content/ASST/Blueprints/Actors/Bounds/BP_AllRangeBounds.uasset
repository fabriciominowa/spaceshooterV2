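; All-range mode boundary volume that turns the player ship around when it begins overlapping the bounds.
; Wall hits, detected by a near-zero impact normal Z, trigger the ship's U-turn if ForceUTurn is set.
; Other hits instantly reverse yaw and negate pitch.
; A DoOnce prevents retriggering until one second after overlap ends, and the construction script applies tags and scale.
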(event OnComponentBeginOverlap(Bounds)
  (params (OverlappedComponent :type Primitive%20Component%20Object%20Reference) (OtherActor :type Actor%20Object%20Reference) (OtherComp :type Primitive%20Component%20Object%20Reference) (OtherBodyIndex :type Integer) (bFromSweep :type Boolean) (SweepResult :type Hit%20Result%20Structure%20%28by%20ref%29))
  ;[1 1 1] Only overlap Player
  (if (Actor|ActorHasTag OtherActor "Player")
    (if (Variables|Setup|GetActive)
      (Utilities|FlowControl|DoOnce false
        (:Completed
          ;[1 1 1] Determine if Player hit a wall (not ceiling)
          (if (Math|Float|NearlyEqual(Float) (Math|Float|Absolute(Float) (.Z (Math|Vector|BreakVector (.ImpactNormal (Collision|BreakHitResult SweepResult))))) 0.0 1e-06)
            (if (Variables|Setup|GetForceUTurn?)
              ;[1 1 1] Perform UTurn
              (bind _asbp_player_ship (Utilities|Casting|CastToBP_PlayerShip OtherActor))
              (Default|EventUTurn _asbp_player_ship)
              (else
                ;[1 1 1] Inverse Player rotation
                (bind _asbp_player_ship_2 (Utilities|Casting|CastToBP_PlayerShip OtherActor :!label _label))
                (Transformation|SetActorRotation _asbp_player_ship_2 (Math|Rotator|Lerp(Rotator) (Transformation|GetWorldRotation (Variables|/Game/ASST/Blueprints/Characters/Player/BP_PlayerShip.BP_PlayerShip_C|GetRoot _asbp_player_ship_2)) (Math|Rotator|MakeRotator (.roll (Transformation|GetWorldRotation (Variables|/Game/ASST/Blueprints/Characters/Player/BP_PlayerShip.BP_PlayerShip_C|GetRoot _asbp_player_ship_2))) (* (.pitch (Transformation|GetWorldRotation (Variables|/Game/ASST/Blueprints/Characters/Player/BP_PlayerShip.BP_PlayerShip_C|GetRoot _asbp_player_ship_2))) -1.0) (+ (.yaw (Transformation|GetWorldRotation (Variables|/Game/ASST/Blueprints/Characters/Player/BP_PlayerShip.BP_PlayerShip_C|GetRoot _asbp_player_ship_2))) 1.8e+02)) 1.0 true) true)))
            (else
              (goto _label))))))))

(event OnComponentEndOverlap(Bounds)
  (params (OverlappedComponent :type Primitive%20Component%20Object%20Reference) (OtherActor :type Actor%20Object%20Reference) (OtherComp :type Primitive%20Component%20Object%20Reference) (OtherBodyIndex :type Integer))
  ;[1 1 1] Only overlap Player
  (if (Actor|ActorHasTag OtherActor "Player")
    (if (Variables|Setup|GetActive)
      (Utilities|FlowControl|Delay 1.0)
      (Utilities|FlowControl|DoOnce false) ; enters at Reset
    )))

(fn ConstructionScript
  (Variables|Default|SetTags (Variables|Default|GetActorTags))
  (Transformation|SetWorldScale3D (Variables|Default|GetBounds) (Variables|Setup|GetBoundScale)))